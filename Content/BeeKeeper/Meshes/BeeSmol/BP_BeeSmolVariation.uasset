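; BP_BeeSmolVariation is a small bee actor that plays a looping animation while cycling through random color variations.
; On BeginPlay it creates a dynamic material instance for the BeeSmol mesh and fills a Species array from the enum, which the graph never reads.
; A looping half-second timer picks a random DT_Icons row and writes its main and secondary colors to the material.
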(event `self.ReceiveBeginPlay`
  (`SkeletalMeshComponent.PlayAnimation` (`self.BeeSmol`) "/Game/BeeKeeper/Meshes/BeeSmol/beesmol_Anim.beesmol_Anim" true)
  (bind _returnvalue (`PrimitiveComponent.CreateDynamicMaterialInstance` (`self.BeeSmol`) 0 "/Game/BeeKeeper/Meshes/BeeSmol/MI_BeeSmal.MI_BeeSmal" "None"))
  (set `self.MIBee` _returnvalue)
  (`|ExecutionSequence`
    (:`then_0`
      (bind _enumvalue (foreach `Species` false)
        (:`LoopBody`
          (`KismetArrayLibrary.Array_Add` (`self.Species`) _enumvalue))))
    (:`then_1`
      (`KismetSystemLibrary.K2_SetTimerDelegate` (delegate `ChangeColor`) 0.5 true))))

(event `ChangeColor`
  (bind _mibee (`self.MIBee`))
  (bind _outrownames (`DataTableFunctionLibrary.GetDataTableRowNames` "/Game/BeeKeeper/BeeModel/DT_Icons.DT_Icons"))
  (bind _returnvalue (`|GetDataTableRow` "/Game/BeeKeeper/BeeModel/DT_Icons.DT_Icons" (`KismetArrayLibrary.Array_Random` _outrownames))
    (:`then`
      (bind (_icon _main _maindark _sec) (break `Icon` _returnvalue))
      (`MaterialInstanceDynamic.SetVectorParameterValue` _mibee "MainColor" (`KismetMathLibrary.Conv_ColorToLinearColor` _main))
      (`MaterialInstanceDynamic.SetVectorParameterValue` _mibee "SecColor" (`KismetMathLibrary.Conv_ColorToLinearColor` _sec)))))

(fn `UserConstructionScript`)