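; VR inventory slot that holds one bee prop, either dropped in by the player or spawned from bee data.
; A sphere trace finds the BP_BeeProp being placed, replacing any current occupant, then attaches it with physics off and PhysicsBody collision ignored.
; Timelines animate the prop into place at small scale and enlarge it while the tracked controller overlaps empty-handed.
; Releasing restores standard scale and collision and clears the slot.
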(event `self.Sphere.OnComponentBeginOverlap`
  (params (OverlappedComponent :type "PrimitiveComponent Object Reference") (OtherActor :type "Actor Object Reference") (OtherComp :type "PrimitiveComponent Object Reference") (OtherBodyIndex :type Integer) (bFromSweep :type Boolean) (SweepResult :type "HitResult Structure (by ref)"))
  (bind _collisioncontrollerref (`self.CollisionControllerRef`))
  (if (== OtherComp _collisioncontrollerref)
    (bind _handempty (`/Game/VRTemplate/Blueprints/VRPawn.HandEmpty` (`self.VRPawnRef`) _collisioncontrollerref))
    (if _handempty
      (`self.ContainedObject`
        (:`then`
          (`self.UpdatePropSacle` (`self.SmallScale`) (`self.StandartScale`)))
        (:`else`)))))

(event `self.Sphere.OnComponentEndOverlap`
  (params (OverlappedComponent :type "PrimitiveComponent Object Reference") (OtherActor :type "Actor Object Reference") (OtherComp :type "PrimitiveComponent Object Reference") (OtherBodyIndex :type Integer))
  (bind _collisioncontrollerref (`self.CollisionControllerRef`))
  (if (== OtherComp _collisioncontrollerref)
    (bind _handempty (`/Game/VRTemplate/Blueprints/VRPawn.HandEmpty` (`self.VRPawnRef`) _collisioncontrollerref))
    (if _handempty
      (bind _containedobject (`self.ContainedObject`)
        (:`then`
          (`self.UpdatePropSacle` (`SceneComponent.RelativeScale3D` (`SceneComponent.GetAttachParent` _containedobject)) (`self.SmallScale`)))
        (:`else`)))))

(event `PushObjectToSlot`
  (params (InitTransform :type "Transform Structure") (EndScale :type "Vector Structure"))
  (bind _itemposition (`self.ItemPosition`))
  (`TimelineComponent.SetPlayRate` (`self.ChangePropTransform`) (/ 1.0 (`self.AnimationRate`)))
  (bind (_direction _alpha) (`Timeline|ChangePropTransform` :!via `PlayFromStart`)
    (:`Update`
      (bind _containedobject (`self.ContainedObject`)
        (:`then`
          (bind _returnvalue (`SceneComponent.GetAttachParent` _containedobject))
          (bind (_returnvalue_location _returnvalue_rotation _returnvalue_scale) (`KismetMathLibrary.BreakTransform` (`KismetMathLibrary.TLerp` InitTransform (`KismetMathLibrary.MakeTransform` (`SceneComponent.K2_GetComponentLocation` _itemposition) (`SceneComponent.K2_GetComponentRotation` _itemposition) EndScale) _alpha)))
          (`SceneComponent.K2_SetWorldLocationAndRotation` _returnvalue _returnvalue_location _returnvalue_rotation false false)
          (`SceneComponent.SetRelativeScale3D` _returnvalue _returnvalue_scale))
        (:`else`)))))

(event `UpdatePropSacle`
  (params (StartScale :type "Vector Structure") (EndScale :type "Vector Structure"))
  (`TimelineComponent.SetPlayRate` (`self.SacleProp`) (/ 1.0 (`self.AnimationRate`)))
  (bind (_direction _alpha) (`Timeline|SacleProp` :!via `PlayFromStart`)
    (:`Update`
      (bind _containedobject (`self.ContainedObject`)
        (:`then`
          (`SceneComponent.SetRelativeScale3D` (`SceneComponent.GetAttachParent` _containedobject) (`KismetMathLibrary.VLerp` StartScale EndScale _alpha)))
        (:`else`)))))

(fn `InitInventorySlot`
  (params (CollisionControllerRef :type "PrimitiveComponent Object Reference") (VrPawn :type "/Game/VRTemplate/Blueprints/VRPawn Object Reference"))
  (set `self.CollisionControllerRef` CollisionControllerRef)
  (set `self.VRPawnRef` VrPawn))

(fn `IsNotContainedObject`
  (params (`Grab Component` :type "/Game/VRTemplate/Blueprints/GrabComponent Object Reference"))
  (returns (Result :type Boolean))
  (return (!= `Grab Component` (`self.ContainedObject`))))

(fn `ReleseContainedObject`
  (params (`Grab Component` :type "/Game/VRTemplate/Blueprints/GrabComponent Object Reference"))
  (returns (IsRelese :type Boolean))
  (locals (Relese :type Boolean))
  (bind _containedobject (`self.ContainedObject`))
  (bind _returnvalue (`SceneComponent.GetAttachParent` _containedobject))
  (`|ExecutionSequence`
    (:`then_0`
      (bind _output_get (set `local.Relese` (== `Grab Component` _containedobject)))
      (if _output_get
        (`SceneComponent.SetRelativeScale3D` _returnvalue (`self.StandartScale`))
        (bind _asprimitive_component (cast `PrimitiveComponent` _returnvalue))
        (`PrimitiveComponent.SetCollisionResponseToChannel` _asprimitive_component "ECC_PhysicsBody" "ECR_Block")
        (set `self.ContainedObject` null)))
    (:`then_1`
      (return _output_get))))

(fn `SetBeeProp`
  (params (Bee :type "BeeGenetic Object Reference"))
  (bind _containedobject (`self.ContainedObject`))
  (bind _itemposition (`self.ItemPosition`))
  (bind _returnvalue (`|SpawnActorFromClass` "/Game/BeeKeeper/Gentic/Blueprints/BP_BeeProp.BP_BeeProp_C" (`KismetMathLibrary.MakeTransform` (`SceneComponent.K2_GetComponentLocation` _itemposition) (`SceneComponent.K2_GetComponentRotation` _itemposition) (0.07 0.07 0.07)) "Undefined" "OverrideRootScale" null true null))
  (`/Game/BeeKeeper/Gentic/Blueprints/BP_BeeProp.UpdateBeeProps` _returnvalue Bee "BeePropInventory")
  (`/Engine/EditorBlueprintResources/StandardMacros.IsValid` _containedobject
    (:`Is Valid`
      (`self.K2_DestroyActor` (`ActorComponent.GetOwner` _containedobject)))
    (:`Is Not Valid`
      _))
  (bind _output_get (set `self.ContainedObject` (`/Game/BeeKeeper/Gentic/Blueprints/BP_BeeProp.GrabComponent` _returnvalue)))
  (`/Game/VRTemplate/Blueprints/GrabComponent.SetPrimitiveCompPhysics` _output_get false)
  (bind _returnvalue_2 (`SceneComponent.GetAttachParent` _output_get))
  (bind _returnvalue_3 (`SceneComponent.K2_AttachToComponent` _returnvalue_2 (`self.DefaultSceneRoot`) "None" "KeepWorld" "KeepWorld" "KeepWorld" true))
  (if _returnvalue_3
    (bind _asprimitive_component (cast `PrimitiveComponent` _returnvalue_2))
    (`PrimitiveComponent.SetCollisionResponseToChannel` _asprimitive_component "ECC_PhysicsBody" "ECR_Ignore")
    (`SceneComponent.SetRelativeScale3D` _returnvalue_2 (`self.SmallScale`))))

(fn `TrySetObject`
  (params (`Grab Component` :type "/Game/VRTemplate/Blueprints/GrabComponent Object Reference"))
  (returns (Sucsess :type Boolean))
  (locals (InitTransform :type "Transform Structure") (IsSucsess :type Boolean))
  (bind _returnvalue (`SceneComponent.K2_GetComponentLocation` (`self.DefaultSceneRoot`)))
  (set `local.IsSucsess` false)
  (bind (_outhits _returnvalue_2) (`KismetSystemLibrary.SphereTraceMultiForObjects` _returnvalue _returnvalue 6.0 (`|MakeArray` "ObjectTypeQuery4" :!type "EObjectTypeQuery Enum")))
  (if _returnvalue_2
    (for _array_element _outhits
      (if (not (`local.IsSucsess`))
        (bind (_bblockinghit _binitialoverlap _time _distance _location _impactpoint _normal _impactnormal _physmat _hitactor) (`GameplayStatics.BreakHitResult` _array_element))
        (cast `/Game/BeeKeeper/Gentic/Blueprints/BP_BeeProp` _hitactor)
        (for _array_element_2 (`self.K2_GetComponentsByClass` _hitactor "/Game/VRTemplate/Blueprints/GrabComponent.GrabComponent_C")
          (if (== `Grab Component` _array_element_2)
            (set `local.IsSucsess` true)
            (bind _containedobject (`self.ContainedObject`)
              (:`then`
                (`self.K2_DestroyActor` (`ActorComponent.GetOwner` _containedobject)))
              (:`else`
                _))
            (bind _output_get (set `self.ContainedObject` `Grab Component`))
            (`/Game/VRTemplate/Blueprints/GrabComponent.SetPrimitiveCompPhysics` _output_get false)
            (bind _returnvalue_3 (`SceneComponent.GetAttachParent` _output_get))
            (bind _returnvalue_4 (`SceneComponent.K2_AttachToComponent` _returnvalue_3 (`self.DefaultSceneRoot`) "None" "KeepWorld" "KeepWorld" "KeepWorld" true))
            (if _returnvalue_4
              (bind _output_get_2 (set `local.InitTransform` (`SceneComponent.K2_GetComponentToWorld` _returnvalue_3)))
              (`self.PushObjectToSlot` (`KismetMathLibrary.MakeTransform` (.location _output_get_2) (.rotation _output_get_2) (`self.StandartScale`)) (`self.SmallScale`))
              (bind _asprimitive_component (cast `PrimitiveComponent` _returnvalue_3))
              (`PrimitiveComponent.SetCollisionResponseToChannel` _asprimitive_component "ECC_PhysicsBody" "ECR_Ignore"))))
        (else
          (break)))))
  (return (`local.IsSucsess`)))

(fn `UserConstructionScript`)