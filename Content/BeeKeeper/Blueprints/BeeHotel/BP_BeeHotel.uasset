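; Bee hotel building that holds bees in eight inventory slots until a release time, then removes them and posts progress messages for their species.
; A looping timer advances per-slot progress and fires ProgressUpdated, which drives particle shutoff and, while the UI is open, widget progress bars.
; Each slot has a pair of Niagara bee effects tinted by species through dynamic materials.
; Bees, slots and progress persist through save data.
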(event `self.ReceiveBeginPlay`
  (bind _defaultsceneroot (`self.DefaultSceneRoot`))
  (bind _beeparticles (`self.BeeParticles`))
  (`|ExecutionSequence`
    (:`then_0`
      (`/Game/BeeKeeper/Blueprints/Outline/BP_OutlineComponent.InitComponent` (`self.BP_OutlineComponent`) (`self.beehotel1`) null)
      (`/Game/BeeKeeper/Inventory/Blueprints/BP_Inventory.InitSlots` (`self.BP_Inventory`) 8 "NewEnumerator1" false)
      (add `/Game/BeeKeeper/Inventory/Blueprints/BP_Inventory.SlotChanged` (`self.BP_Inventory`) (delegate `SlotChanged`))
      (for _ (range 1 (+ (`KismetArrayLibrary.Array_Length` (`/Game/BeeKeeper/Inventory/Blueprints/BP_Inventory.Slots` (`self.BP_Inventory`))) 1))
        (`KismetArrayLibrary.Array_Add` (`self.BeesProgressTime`)))
      (`KismetSystemLibrary.K2_SetTimerDelegate` (delegate `TickBees`) (`self.BeeHotelDelta`) true))
    (:`then_1`
      (bind _enumvalue (foreach `Species` false)
        (:`LoopBody`
          (`KismetArrayLibrary.Array_Add` (`self.AllSpecies`) _enumvalue))
        (:`then`
          (add `self.ProgressUpdated` (delegate `DeactivateParticle`))
          (add `/Game/BeeKeeper/Inventory/Blueprints/BP_Inventory.SlotChanged` (`self.BP_Inventory`) (delegate `ShowParicleBees`)))))
    (:`then_2`
      (bind _returnvalue (`KismetMaterialLibrary.CreateDynamicMaterialInstance` "/Game/BeeKeeper/Meshes/BeeSmol/MI_BeeSmal.MI_BeeSmal"))
      (bind _output_get (set `self.MIBee` _returnvalue))
      (for _array_element (`self.ParticleLocations`)
        (bind _asbp_bee_game_instance (cast `/Game/BeeKeeper/Blueprints/BP_BeeGameInstance` (`GameplayStatics.GetGameInstance`)))
        (bind _dmi (`/Game/BeeKeeper/Blueprints/BP_BeeGameInstance.GetDMIBeeParticle` _asbp_bee_game_instance (`KismetArrayLibrary.Array_Random` (`self.AllSpecies`))))
        (bind _returnvalue_2 (`NiagaraFunctionLibrary.SpawnSystemAttached` "/Game/BeeKeeper/FX/NS_MoveAround.NS_MoveAround" _defaultsceneroot "None" _array_element (struct) "KeepRelativeOffset"))
        (`NiagaraComponent.SetVariableMaterial` _returnvalue_2 "BeeMat" _dmi)
        (bind _returnvalue_3 (`NiagaraFunctionLibrary.SpawnSystemAttached` "/Game/BeeKeeper/FX/NS_MoveAround.NS_MoveAround" _defaultsceneroot "None" (- _array_element (0.0 42.0 0.0)) (struct :`Yaw` 180.0) "KeepRelativeOffset"))
        (`NiagaraComponent.SetVariableMaterial` _returnvalue_3 "BeeMat" _dmi)
        (`KismetArrayLibrary.Array_Add` _beeparticles _returnvalue_2)
        (`KismetArrayLibrary.Array_Add` _beeparticles _returnvalue_3)
        (`ActorComponent.Deactivate` _returnvalue_2)
        (`ActorComponent.Deactivate` _returnvalue_3))
      (bind _outrownames (`DataTableFunctionLibrary.GetDataTableRowNames` "/Game/BeeKeeper/BeeModel/DT_Icons.DT_Icons"))
      (bind _returnvalue_4 (`|GetDataTableRow` "/Game/BeeKeeper/BeeModel/DT_Icons.DT_Icons" (`KismetArrayLibrary.Array_Random` _outrownames))
        (:`then`
          (bind (_icon _main _maindark _sec) (break `Icon` _returnvalue_4))
          (`MaterialInstanceDynamic.SetVectorParameterValue` (`self.MIBee`) "MainColor" (`KismetMathLibrary.Conv_ColorToLinearColor` _main))
          (`MaterialInstanceDynamic.SetVectorParameterValue` (`self.MIBee`) "SecColor" (`KismetMathLibrary.Conv_ColorToLinearColor` _sec)))))))

(event `TickBees`
  (bind _returnvalue (`GameplayStatics.GetGameInstance`))
  (bind _bp_inventory (`self.BP_Inventory`))
  (bind _slots (`/Game/BeeKeeper/Inventory/Blueprints/BP_Inventory.Slots` _bp_inventory))
  (bind (_arrayelement _arrayindex) (`/Game/BeeKeeper/Blueprints/BPM_Utils.ForEachLoop_ByRef` (`self.BeesProgressTime`))
    (:`LoopBody`
      (bind (_type _inventoryidx) (break `/Game/BeeKeeper/Blueprints/Inventory/S_SlotData` (`|GetArrayItem` (`/Game/BeeKeeper/Inventory/Blueprints/BP_Inventory.Slots` (`self.BP_Inventory`)) _arrayindex)))
      (if (!= _inventoryidx -1)
        (`|VariableSetRef` _arrayelement (+ _arrayelement (`self.BeeHotelDelta`)))
        (`self.ProgressUpdated` _arrayindex)
        (if (> _arrayelement (`self.BeeReleaseTime`))
          (`|ExecutionSequence`
            (:`then_0`
              (bind _output (`|GetArrayItem` (`/Game/BeeKeeper/Inventory/Blueprints/BP_Inventory.Bees` (`self.BP_Inventory`)) _inventoryidx))
              (bind _main (`BeeGenetic.Main` _output))
              (message `/Game/BeeKeeper/Blueprints/BPI_GameInstanceTransfer.AddBeeProgress` _returnvalue _main)
              (bind _sec (`BeeGenetic.Sec` _output))
              (if (`|EnumInequality` _main _sec)
                (message `/Game/BeeKeeper/Blueprints/BPI_GameInstanceTransfer.AddBeeProgress` _returnvalue _sec)))
            (:`then_1`
              (`KismetArrayLibrary.Array_Remove` (`/Game/BeeKeeper/Inventory/Blueprints/BP_Inventory.Bees` (`self.BP_Inventory`)) _inventoryidx)
              (`/Game/BeeKeeper/Inventory/Blueprints/BP_Inventory.UpdateSlotsIdxAfterRemove` _bp_inventory _slots "NewEnumerator1" _inventoryidx)
              (setmembers `/Game/BeeKeeper/Blueprints/Inventory/S_SlotData` :`StructRef` (`|GetArrayItem` _slots _arrayindex) :`InventoryIdx` -1)
              (bind _asbp_first_person_controller (cast `/Game/BeeKeeper/Blueprints/FirstPersonController/BP_FirstPersonController` (`GameplayStatics.GetPlayerCharacter` 0)))
              (bind _wb_beehiveselect (`/Game/BeeKeeper/UI/WB_HandInventory.WB_BeeHiveSelect` (`/Game/BeeKeeper/Blueprints/FirstPersonController/BP_FirstPersonController.WB_HandInventoryRef` _asbp_first_person_controller)))
              ;[1 1 1] TODO: also perfectly in info panel check displayed idx slot or inventory, then hide data if it selected idx
              (if (and (`Widget.IsVisible` _wb_beehiveselect) (== (`/Game/BeeKeeper/UI/WB_BeeHiveSelect.BuildingInventory` _wb_beehiveselect) (`self.BP_Inventory`)))
                ;;[1 1 1] TODO: select first correct or hide frame
                (`/Game/BeeKeeper/UI/WB_BeeHiveSelect.ClearSlot` _wb_beehiveselect _arrayindex)))))))))

(event `SlotChanged`
  (params (Idx :type Integer))
  (if (!= (`.InventoryIdx_5_579F21AC4D8636E5B62930970C700287` (break `/Game/BeeKeeper/Blueprints/Inventory/S_SlotData` (`|GetArrayItem` (`/Game/BeeKeeper/Inventory/Blueprints/BP_Inventory.Slots` (`self.BP_Inventory`)) Idx))) -1)
    (bind _asbp_first_person_controller (cast `/Game/BeeKeeper/Blueprints/FirstPersonController/BP_FirstPersonController` (`GameplayStatics.GetPlayerCharacter` 0)))
    (`KismetArrayLibrary.Array_Set` (`self.BeesProgressTime`) Idx)
    (bind _progressbar (`/Game/BeeKeeper/UI/WB_HexSlot.ProgressBar` (`|GetArrayItem` (`/Game/BeeKeeper/UI/WB_BeeHiveSelect.Slots` (`/Game/BeeKeeper/UI/WB_HandInventory.WB_BeeHiveSelect` (`/Game/BeeKeeper/Blueprints/FirstPersonController/BP_FirstPersonController.WB_HandInventoryRef` _asbp_first_person_controller))) Idx)))
    ;[1 1 1] TODO: move this to widget func
    (`Widget.SetVisibility` _progressbar "SelfHitTestInvisible")
    (`ProgressBar.SetPercent` _progressbar 0.0)))

(event `DeactivateParticle` :!signature `self.ProgressUpdated`
  (params (SlotIdx :type Integer))
  (if (> (`|GetArrayItem` (`self.BeesProgressTime`) SlotIdx) (`self.BeeReleaseTime`))
    (`self.DeactivateBeesParticles` SlotIdx)))

(event `/Game/BeeKeeper/Blueprints/Interactable/BPI_Interactable.Interact`
  (bind _asbp_first_person_controller (cast `/Game/BeeKeeper/Blueprints/FirstPersonController/BP_FirstPersonController` (`GameplayStatics.GetPlayerCharacter` 0)))
  (`/Game/BeeKeeper/Blueprints/FirstPersonController/BP_FirstPersonController.ToggleInveontory` _asbp_first_person_controller "NewEnumerator0"))

(event `ShowParicleBees`
  (params (Idx :type Integer))
  (bind _returnvalue (* Idx 2))
  (bind _bp_inventory (`self.BP_Inventory`))
  (bind _beeparticles (`self.BeeParticles`))
  (bind _output (`|GetArrayItem` _beeparticles _returnvalue))
  (bind _output_2 (`|GetArrayItem` _beeparticles (+ _returnvalue 1)))
  (if (`/Game/BeeKeeper/Blueprints/BPF_Utils.Has Slot Item` (`|GetArrayItem` (`/Game/BeeKeeper/Inventory/Blueprints/BP_Inventory.Slots` (`self.BP_Inventory`)) Idx))
    (bind _asbp_bee_game_instance (cast `/Game/BeeKeeper/Blueprints/BP_BeeGameInstance` (`GameplayStatics.GetGameInstance`)))
    (bind _dmi (`/Game/BeeKeeper/Blueprints/BP_BeeGameInstance.GetDMIBeeParticle` _asbp_bee_game_instance (`BeeGenetic.Main` (`|GetArrayItem` (`/Game/BeeKeeper/Inventory/Blueprints/BP_Inventory.Bees` _bp_inventory) (`.InventoryIdx_5_579F21AC4D8636E5B62930970C700287` (break `/Game/BeeKeeper/Blueprints/Inventory/S_SlotData` (`|GetArrayItem` (`/Game/BeeKeeper/Inventory/Blueprints/BP_Inventory.Slots` _bp_inventory) Idx)))))))
    (`NiagaraComponent.SetVariableMaterial` _output "BeeMat" _dmi)
    (`NiagaraComponent.SetVariableMaterial` _output_2 "BeeMat" _dmi)
    (`ActorComponent.Activate` _output false)
    (`ActorComponent.Activate` _output_2 false)
    (else
      (`self.DeactivateBeesParticles` Idx))))

(event `/Game/BeeKeeper/Blueprints/Interactable/BPI_Interactable.SwitchUiAfterIneract`
  (params (IsUiModeActive :type Boolean))
  (if IsUiModeActive
    (bind _asbp_first_person_controller (cast `/Game/BeeKeeper/Blueprints/FirstPersonController/BP_FirstPersonController` (`GameplayStatics.GetPlayerCharacter` 0)))
    (bind _wb_handinventoryref (`/Game/BeeKeeper/Blueprints/FirstPersonController/BP_FirstPersonController.WB_HandInventoryRef` _asbp_first_person_controller))
    (bind _wb_inventory (`/Game/BeeKeeper/UI/WB_HandInventory.WB_Inventory` _wb_handinventoryref))
    (`/Game/BeeKeeper/UI/WB_Inventory.DisplayBees` _wb_inventory)
    (`/Game/BeeKeeper/UI/WB_Inventory.SwitchSelectTypes` _wb_inventory false)
    (`/Game/BeeKeeper/UI/WB_BeeHiveSelect.DisplayBeehotelSlots` (`/Game/BeeKeeper/UI/WB_HandInventory.WB_BeeHiveSelect` _wb_handinventoryref))
    (add `self.ProgressUpdated` (delegate `UpdatePrecentage`))
    (for _array_element (`/Game/BeeKeeper/Inventory/Blueprints/BP_Inventory.Slots` (`self.BP_Inventory`))
      (if (!= (`.InventoryIdx_5_579F21AC4D8636E5B62930970C700287` (break `/Game/BeeKeeper/Blueprints/Inventory/S_SlotData` _array_element)) -1)
        (`self.ProgressUpdated` 0)))
    (else
      (remove `self.ProgressUpdated` (delegate `UpdatePrecentage`)))))

(event `UpdatePrecentage` :!signature `self.ProgressUpdated`
  (params (SlotIdx :type Integer))
  (bind _asbp_first_person_controller (cast `/Game/BeeKeeper/Blueprints/FirstPersonController/BP_FirstPersonController` (`GameplayStatics.GetPlayerCharacter` 0)))
  (`ProgressBar.SetPercent` (`/Game/BeeKeeper/UI/WB_HexSlot.ProgressBar` (`|GetArrayItem` (`/Game/BeeKeeper/UI/WB_BeeHiveSelect.Slots` (`/Game/BeeKeeper/UI/WB_HandInventory.WB_BeeHiveSelect` (`/Game/BeeKeeper/Blueprints/FirstPersonController/BP_FirstPersonController.WB_HandInventoryRef` _asbp_first_person_controller))) SlotIdx)) (/ (`|GetArrayItem` (`self.BeesProgressTime`) SlotIdx) (`self.BeeReleaseTime`))))

(event `/Game/BeeKeeper/Blueprints/PlayerBase/BPI_Buildings.SaveBuildingData`
  (bind _asbp_bee_game_instance (cast `/Game/BeeKeeper/Blueprints/BP_BeeGameInstance` (`GameplayStatics.GetGameInstance`)))
  (bind _beesdata (`/Game/BeeKeeper/Blueprints/BPF_Utils.GetBeesDataFromBees` (`/Game/BeeKeeper/Inventory/Blueprints/BP_Inventory.Bees` (`self.BP_Inventory`))))
  (`KismetArrayLibrary.Array_Add` (`/Game/BeeKeeper/Blueprints/SaveGame/BP_SaveGame.BeeHotelSave` (`/Game/BeeKeeper/Blueprints/BP_BeeGameInstance.SaveData` _asbp_bee_game_instance)) (make `/Game/BeeKeeper/Blueprints/SaveGame/S_BeeHotelSaveData` _beesdata (`/Game/BeeKeeper/Inventory/Blueprints/BP_Inventory.Slots` (`self.BP_Inventory`)) (`self.GetTransform`) (`self.BeesProgressTime`))))

(fn `DeactivateBeesParticles`
  (params (SlotIdx :type Integer))
  (bind _returnvalue (* SlotIdx 2))
  (bind _beeparticles (`self.BeeParticles`))
  (`ActorComponent.Deactivate` (`|GetArrayItem` _beeparticles _returnvalue))
  (`ActorComponent.Deactivate` (`|GetArrayItem` _beeparticles (+ _returnvalue 1))))

(fn `Inspect`
  (returns (Yes :type Boolean))
  (return false))

(fn `IsBuilding`
  (returns (Building :type Boolean))
  (return true))

(fn `IsInspectable`
  (returns (Yes :type Boolean))
  (return false))

(fn `LoadFromSaveFile`
  (params (Save :type "/Game/BeeKeeper/Blueprints/SaveGame/S_BeeHotelSaveData Structure"))
  (bind (_bees _slots _transform _beesprogress) (break `/Game/BeeKeeper/Blueprints/SaveGame/S_BeeHotelSaveData` Save))
  (`|ExecutionSequence`
    (:`then_0`
      ;[1 1 1] TODO: move this to utlis
      (for _array_element _bees
        (bind _returnvalue (`BeeGenetic.Construct` (break `/Game/BeeKeeper/Blueprints/SaveGame/S_BeeSaveData` _array_element) (`.Sec_5_C70A1CC548EDFF1A1775FE9F61A6EAE7` (break `/Game/BeeKeeper/Blueprints/SaveGame/S_BeeSaveData` _array_element)) (`.Speed_8_1CD6901A441796C254201C907A2497F4` (break `/Game/BeeKeeper/Blueprints/SaveGame/S_BeeSaveData` _array_element)) (`.Fertility_10_F818F0FA45FF2E27C128FE84F2FF8922` (break `/Game/BeeKeeper/Blueprints/SaveGame/S_BeeSaveData` _array_element))))
        (`KismetArrayLibrary.Array_Add` (`/Game/BeeKeeper/Inventory/Blueprints/BP_Inventory.Bees` (`self.BP_Inventory`)) _returnvalue)))
    (:`then_1`
      (set `/Game/BeeKeeper/Inventory/Blueprints/BP_Inventory.Slots` _slots (`self.BP_Inventory`))
      (if (`KismetArrayLibrary.Array_IsNotEmpty` _beesprogress)
        (set `self.BeesProgressTime` _beesprogress)))
    (:`then_2`
      (`ActorComponent.Activate` (`self.NS_MoveAround`) false))))

(fn `UserConstructionScript`)