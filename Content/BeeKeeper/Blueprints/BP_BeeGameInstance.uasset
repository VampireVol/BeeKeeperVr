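; Game instance for the beekeeping game, holding money, placed buildings, species discovery, research effects and the BP_SaveGame slot.
; Saving gathers VR or first-person inventory, buildings, bee props and restored hives; loading respawns buildings into a map keyed by hex coordinates.
; Completed research calls same-named functions by string to upgrade hive capacity, enable gene speed or advance restoration stages.
; It also computes hive income, checks end goals and caches per-species particle materials.
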(event `self.ReceiveInit`)

(event `/Game/BeeKeeper/Blueprints/SaveGame/BPI_SaveGameData.LoadGameData`
  (`|ExecutionSequence`
    (:`then_0`
      (bind _returnvalue (`GameplayStatics.DoesSaveGameExist` (`self.SaveSlotName`)))
      (if _returnvalue
        (bind _returnvalue_2 (`GameplayStatics.LoadGameFromSlot` (`self.SaveSlotName`)))
        (bind _asbp_save_game (cast `/Game/BeeKeeper/Blueprints/SaveGame/BP_SaveGame` _returnvalue_2))
        (set `self.SaveData` _asbp_save_game)
        (else
          (bind _returnvalue_3 (`|GenericCreateObject` "/Game/BeeKeeper/Blueprints/SaveGame/BP_SaveGame.BP_SaveGame_C"))
          (set `self.SaveData` _returnvalue_3))))
    (:`then_1`
      (`self.LoadInstanceDataFromSave`))))

(event `/Game/BeeKeeper/Blueprints/SaveGame/BPI_SaveGameData.SaveGameData`
  (`GameplayStatics.SaveGameToSlot` (`self.SaveData`) (`self.SaveSlotName`)))

(event `/Game/BeeKeeper/Blueprints/SaveGame/BPI_SaveGameData.SavePlayer`
  (params (PlayerData :type "/Game/BeeKeeper/Blueprints/SaveGame/S_PlayerSave Structure"))
  (bind _savedata (`self.SaveData`))
  (bind _savedata_2 (`self.SaveData`))
  (`|ExecutionSequence`
    (:`then_0`
      (set `/Game/BeeKeeper/Blueprints/SaveGame/BP_SaveGame.PlayerSave` PlayerData (`self.SaveData`))
      (if (`HeadMountedDisplayFunctionLibrary.IsHeadMountedDisplayEnabled`)
        (bind _asvrpawn (cast `/Game/VRTemplate/Blueprints/VRPawn` (`GameplayStatics.GetPlayerPawn` 0)))
        (bind (_bees _frames _items) (`/Game/BeeKeeper/Inventory/Blueprints/BP_Inventory.Get Inventory Save Data` (`/Game/VRTemplate/Blueprints/VRPawn.BP_Inventory` _asvrpawn)))
        (set `/Game/BeeKeeper/Blueprints/SaveGame/BP_SaveGame.BeesSave` _bees _savedata_2)
        (set `/Game/BeeKeeper/Blueprints/SaveGame/BP_SaveGame.FramesSave` _frames _savedata_2)
        (set `/Game/BeeKeeper/Blueprints/SaveGame/BP_SaveGame.ItemsSave` _items _savedata_2)
        (else
          (bind _asbp_first_person_controller (cast `/Game/BeeKeeper/Blueprints/FirstPersonController/BP_FirstPersonController` (`GameplayStatics.GetPlayerCharacter` 0)))
          (bind (_bees_2 _frames_2 _items_2) (`/Game/BeeKeeper/Inventory/Blueprints/BP_Inventory.Get Inventory Save Data` (`/Game/BeeKeeper/Blueprints/FirstPersonController/BP_FirstPersonController.BP_Inventory` _asbp_first_person_controller)))
          (set `/Game/BeeKeeper/Blueprints/SaveGame/BP_SaveGame.BeesSave` _bees_2 _savedata)
          (set `/Game/BeeKeeper/Blueprints/SaveGame/BP_SaveGame.FramesSave` _frames_2 _savedata)
          (set `/Game/BeeKeeper/Blueprints/SaveGame/BP_SaveGame.ItemsSave` _items_2 _savedata))))
    (:`then_1`
      (`self.ClearSaveArrays`)
      (bind _values (`BlueprintMapLibrary.Map_Values` (`self.Buildings`)))
      (for _array_element _values
        (message `/Game/BeeKeeper/Blueprints/PlayerBase/BPI_Buildings.SaveBuildingData` _array_element)))
    (:`then_2`
      (set `/Game/BeeKeeper/Blueprints/SaveGame/BP_SaveGame.Money` (`self.Money`) (`self.SaveData`)))
    (:`then_3`
      (`KismetArrayLibrary.Array_Clear` (`/Game/BeeKeeper/Blueprints/SaveGame/BP_SaveGame.BeePropsSave` (`self.SaveData`)))
      (bind _outactors (`GameplayStatics.GetAllActorsOfClassWithTag` "/Game/BeeKeeper/Gentic/Blueprints/BP_BeeProp.BP_BeeProp_C" "BeeProp"))
      (for _array_element_2 _outactors
        (bind _beegenetic (`/Game/BeeKeeper/Gentic/Blueprints/BP_BeeProp.BeeGenetic` _array_element_2))
        (`KismetArrayLibrary.Array_Add` (`/Game/BeeKeeper/Blueprints/SaveGame/BP_SaveGame.BeePropsSave` (`self.SaveData`)) (make `/Game/BeeKeeper/Blueprints/SaveGame/S_BeePropSaveData` (`Actor.GetTransform` _array_element_2) (make `/Game/BeeKeeper/Blueprints/SaveGame/S_BeeSaveData` (`BeeGenetic.Main` _beegenetic) (`BeeGenetic.Sec` _beegenetic) (`BeeGenetic.Speed` _beegenetic) (`BeeGenetic.Fertility` _beegenetic))))))
    (:`then_4`
      (`KismetArrayLibrary.Array_Clear` (`/Game/BeeKeeper/Blueprints/SaveGame/BP_SaveGame.DiscoveredSpecies` (`self.SaveData`)))
      (bind _enumvalue (foreach `Species` false)
        (:`LoopBody`
          (bind _returnvalue (`BeeGenetic.IsDiscoveredSpecies` _enumvalue))
          (if _returnvalue
            (`KismetArrayLibrary.Array_Add` (`/Game/BeeKeeper/Blueprints/SaveGame/BP_SaveGame.DiscoveredSpecies` (`self.SaveData`)) _enumvalue)))))
    (:`then_5`
      (bind _outactors_2 (`GameplayStatics.GetAllActorsOfClass` "/Game/BeeKeeper/Blueprints/RestoredHive/BP_RestoredHive.BP_RestoredHive_C"))
      (for _array_element_3 _outactors_2
        (bind _save (`/Game/BeeKeeper/Blueprints/RestoredHive/BP_RestoredHive.GetRestoredHiveSaveData` _array_element_3))
        (`KismetArrayLibrary.Array_Add` (`/Game/BeeKeeper/Blueprints/SaveGame/BP_SaveGame.RestoredHives` (`self.SaveData`)) _save)))))

(event `/Game/BeeKeeper/Blueprints/BPI_GameInstanceTransfer.AddBeeProgress`
  (params (Type :type "Species Enum" :default "Meadow"))
  (bind _beerestoreprogress (`self.BeeRestoreProgress`))
  (bind (_value _returnvalue) (`BlueprintMapLibrary.Map_Find` _beerestoreprogress Type))
  (if _returnvalue
    (`BlueprintMapLibrary.Map_Add` (`self.BeeRestoreProgress`) Type (+ _value 1))
    (else
      (`BlueprintMapLibrary.Map_Add` _beerestoreprogress Type 1)))
  (`KismetSystemLibrary.PrintText` (`|FormatText` "Progess for species: {0} {1}" (`|GetEnumeratorNameAsString` Type) (`BlueprintMapLibrary.Map_Find` (`self.BeeRestoreProgress`) Type))))

(event `/Game/BeeKeeper/Blueprints/BPI_GameInstanceTransfer.ResearchComplete`
  (params (ResearchName :type Name))
  (`BeeFunctionLibrary.CallFunctionByName` null ResearchName))

(fn `BeehiveCapacity1`
  (`self.ResearchBeehiveCapacity` 4))

(fn `BeehiveCapacity2`
  (`self.ResearchBeehiveCapacity` 5))

(fn `BeehiveCapacity3`
  (`self.ResearchBeehiveCapacity` 6))

(fn `CheckEndGoals`
  (returns (GameFinished :type Boolean))
  (bind _returnvalue (`BeeGenetic.DiscoveredCount`))
  (return (and (> (`self.Money`) 1000000) (== _returnvalue (enumcount `Species`)))))

(fn `ClearBeeProps`
  (locals (ClearTags :type "Array of Name"))
  (for _array_element (`local.ClearTags`)
    (bind _outactors (`GameplayStatics.GetAllActorsOfClassWithTag` "/Game/BeeKeeper/Gentic/Blueprints/BP_BeeProp.BP_BeeProp_C" _array_element))
    (for _array_element_2 _outactors
      (`Actor.K2_DestroyActor` _array_element_2))))

(fn `ClearGameState`
  (`self.ClearInstanceData`)
  (`BeeGenetic.ClearDiscoveredSpecies`)
  (`self.ClearBeeProps`))

(fn `ClearInstanceData`
  (set `self.Money` 0)
  (bind _values (`BlueprintMapLibrary.Map_Values` (`self.Buildings`)))
  (for _array_element _values
    (`Actor.K2_DestroyActor` _array_element))
  (`BlueprintMapLibrary.Map_Clear` (`self.Buildings`)))

(fn `ClearSaveArrays`
  (bind _savedata (`self.SaveData`))
  (`KismetArrayLibrary.Array_Clear` (`/Game/BeeKeeper/Blueprints/SaveGame/BP_SaveGame.BeeHivesSave` _savedata))
  (`KismetArrayLibrary.Array_Clear` (`/Game/BeeKeeper/Blueprints/SaveGame/BP_SaveGame.CentrifugeSave` _savedata))
  (`KismetArrayLibrary.Array_Clear` (`/Game/BeeKeeper/Blueprints/SaveGame/BP_SaveGame.BeeHotelSave` _savedata))
  (`KismetArrayLibrary.Array_Clear` (`/Game/BeeKeeper/Blueprints/SaveGame/BP_SaveGame.ExtractorDNASave` _savedata))
  (`KismetArrayLibrary.Array_Clear` (`/Game/BeeKeeper/Blueprints/SaveGame/BP_SaveGame.RestoredHives` _savedata)))

(fn `GetDMIBeeParticle`
  (params (Type :type "Species Enum" :default "Meadow"))
  (returns (DMI :type "MaterialInstanceDynamic Object Reference"))
  (bind _beesmaterials (`self.BeesMaterials`))
  (bind (_value _returnvalue) (`BlueprintMapLibrary.Map_Find` _beesmaterials Type))
  (if _returnvalue
    (return _value)
    (else
      (bind _returnvalue_2 (`KismetMaterialLibrary.CreateDynamicMaterialInstance` "/Game/BeeKeeper/Meshes/BeeSmol/MI_BeeSmalParticle.MI_BeeSmalParticle"))
      (`BlueprintMapLibrary.Map_Add` _beesmaterials Type _returnvalue_2)
      (bind _returnvalue_3 (`|GetDataTableRow` "/Game/BeeKeeper/BeeModel/DT_Icons.DT_Icons" (`|GetEnumeratorName` Type))
        (:`then`
          (bind (_icon _main _maindark _sec) (break `Icon` _returnvalue_3))
          (`MaterialInstanceDynamic.SetVectorParameterValue` _returnvalue_2 "MainColor" (`KismetMathLibrary.Conv_ColorToLinearColor` _main))
          (`MaterialInstanceDynamic.SetVectorParameterValue` _returnvalue_2 "SecColor" (`KismetMathLibrary.Conv_ColorToLinearColor` _sec))
          (return _returnvalue_2))))))

(fn `GetFrameIdx`
  (returns (Idx :type Integer))
  (locals (Out :type Integer))
  (bind _savedata (`self.SaveData`)
    (:`then`
      (bind _framecount (`/Game/BeeKeeper/Blueprints/SaveGame/BP_SaveGame.FrameCount` _savedata))
      (set `local.Out` _framecount)
      (set `/Game/BeeKeeper/Blueprints/SaveGame/BP_SaveGame.FrameCount` (+ _framecount 1) _savedata)
      (return (`local.Out`)))
    (:`else`
      ; Todo: maybe better load save for save count when beehive frame beginplay
      (return 0))))

(fn `GetMoney`
  (params (Dt :type "Float (double-precision)"))
  (returns (Money :type Integer64) (IncomeValuePerMin :type Integer))
  (locals (`Income Value Per Min` :type Integer))
  (bind _values (`BlueprintMapLibrary.Map_Values` (`self.Buildings`)))
  (for _array_element _values
    (bind _asbp_bee_hive (cast `/Game/BeeKeeper/BeeHive/BP_BeeHive` _array_element))
    (bind _incomevalue (`/Game/BeeKeeper/UI/WB_BeeHiveStats.IncomeValue` (`/Game/BeeKeeper/BeeHive/BP_BeeHive.Bee Hive Stats WB` _asbp_bee_hive)))
    (set `self.Money` (+ (`KismetMathLibrary.Round64` (* (* (/ (`KismetMathLibrary.Conv_IntToDouble` _incomevalue) 60.0) 100.0) Dt)) (`self.Money`)))
    (set `local.Income Value Per Min` (+ _incomevalue (`local.Income Value Per Min`))))
  (return (`self.Money`) (`local.Income Value Per Min`)))

(fn `GetSaveGameData`
  (returns (SaveData :type "/Game/BeeKeeper/Blueprints/SaveGame/BP_SaveGame Object Reference"))
  (return (`self.SaveData`)))

(fn `I_IsSavesExists`
  (returns (Exists :type Boolean))
  (bind _returnvalue (`GameplayStatics.DoesSaveGameExist` (`self.SaveSlotName`)))
  (return _returnvalue))

(fn `LoadInstanceDataFromSave`
  (`|ExecutionSequence`
    (:`then_0`
      (`self.ClearInstanceData`)
      (set `self.Money` (`/Game/BeeKeeper/Blueprints/SaveGame/BP_SaveGame.Money` (`self.SaveData`)))
      (`self.ClearBeeProps`)
      (for _array_element (`/Game/BeeKeeper/Blueprints/SaveGame/BP_SaveGame.BeeHivesSave` (`self.SaveData`))
        (bind _returnvalue (`|SpawnActorFromClass` "/Game/BeeKeeper/BeeHive/BP_BeeHive.BP_BeeHive_C" (`.Transform_10_B8BC53D1448C7316490CC5A5F04872EE` (break `/Game/BeeKeeper/Blueprints/SaveGame/S_BeeHiveSaveData` _array_element)) "Undefined" "OverrideRootScale" null false null))
        (`/Game/BeeKeeper/BeeHive/BP_BeeHive.LoadBeeHiveFromSaveData` _returnvalue _array_element)
        (bind (_returnvalue_x _returnvalue_y) (`KismetMathLibrary.BreakVector` (`Actor.K2_GetActorLocation` _returnvalue)))
        (bind (_q _r) (`/Game/BeeKeeper/BeeHive/BP_GridLibrary.PixelToHex` _returnvalue_x _returnvalue_y))
        (`BlueprintMapLibrary.Map_Add` (`self.Buildings`) (`KismetMathLibrary.MakeVector2D` (`KismetMathLibrary.Conv_IntToDouble` _q) (`KismetMathLibrary.Conv_IntToDouble` _r)) _returnvalue))
      (for _array_element_2 (`/Game/BeeKeeper/Blueprints/SaveGame/BP_SaveGame.CentrifugeSave` (`self.SaveData`))
        (bind _returnvalue_2 (`|SpawnActorFromClass` "/Game/BeeKeeper/Blueprints/Centrifuge/BP_Centrifuge.BP_Centrifuge_C" (`.Transform_5_6FC3C8B24A685FE8F1B05192C8AC808A` (break `/Game/BeeKeeper/Blueprints/SaveGame/S_CentrifugeSaveData` _array_element_2)) "Undefined" "OverrideRootScale" null null))
        (`/Game/BeeKeeper/Blueprints/Centrifuge/BP_Centrifuge.LoadFromSaveFile` _returnvalue_2 _array_element_2)
        (bind (_returnvalue_x_2 _returnvalue_y_2) (`KismetMathLibrary.BreakVector` (`Actor.K2_GetActorLocation` _returnvalue_2)))
        (bind (_q_2 _r_2) (`/Game/BeeKeeper/BeeHive/BP_GridLibrary.PixelToHex` _returnvalue_x_2 _returnvalue_y_2))
        (`BlueprintMapLibrary.Map_Add` (`self.Buildings`) (`KismetMathLibrary.MakeVector2D` (`KismetMathLibrary.Conv_IntToDouble` _q_2) (`KismetMathLibrary.Conv_IntToDouble` _r_2)) _returnvalue_2))
      (for _array_element_3 (`/Game/BeeKeeper/Blueprints/SaveGame/BP_SaveGame.BeeHotelSave` (`self.SaveData`))
        (bind _returnvalue_3 (`|SpawnActorFromClass` "/Game/BeeKeeper/Blueprints/BeeHotel/BP_BeeHotel.BP_BeeHotel_C" (`.Transform_2_15907FA04D3AF4409F7E97830F6423AB` (break `/Game/BeeKeeper/Blueprints/SaveGame/S_BeeHotelSaveData` _array_element_3)) "Undefined" "OverrideRootScale" null null))
        (`/Game/BeeKeeper/Blueprints/BeeHotel/BP_BeeHotel.LoadFromSaveFile` _returnvalue_3 _array_element_3)
        (bind (_returnvalue_x_3 _returnvalue_y_3) (`KismetMathLibrary.BreakVector` (`Actor.K2_GetActorLocation` _returnvalue_3)))
        (bind (_q_3 _r_3) (`/Game/BeeKeeper/BeeHive/BP_GridLibrary.PixelToHex` _returnvalue_x_3 _returnvalue_y_3))
        (`BlueprintMapLibrary.Map_Add` (`self.Buildings`) (`KismetMathLibrary.MakeVector2D` (`KismetMathLibrary.Conv_IntToDouble` _q_3) (`KismetMathLibrary.Conv_IntToDouble` _r_3)) _returnvalue_3))
      (for _array_element_4 (`/Game/BeeKeeper/Blueprints/SaveGame/BP_SaveGame.ExtractorDNASave` (`self.SaveData`))
        (bind _returnvalue_4 (`|SpawnActorFromClass` "/Game/BeeKeeper/Blueprints/ExtractorDNA/BP_ExtractorDNA.BP_ExtractorDNA_C" (`.Transform_3_1CC5432A4A8F0FBF3ABF4193E97E33BB` (break `/Game/BeeKeeper/Blueprints/SaveGame/S_ExtractorDNASave` _array_element_4)) "Undefined" "OverrideRootScale" null null))
        (`/Game/BeeKeeper/Blueprints/ExtractorDNA/BP_ExtractorDNA.LoadFromSaveFile` _returnvalue_4 _array_element_4)
        (bind (_returnvalue_x_4 _returnvalue_y_4) (`KismetMathLibrary.BreakVector` (`Actor.K2_GetActorLocation` _returnvalue_4)))
        (bind (_q_4 _r_4) (`/Game/BeeKeeper/BeeHive/BP_GridLibrary.PixelToHex` _returnvalue_x_4 _returnvalue_y_4))
        (`BlueprintMapLibrary.Map_Add` (`self.Buildings`) (`KismetMathLibrary.MakeVector2D` (`KismetMathLibrary.Conv_IntToDouble` _q_4) (`KismetMathLibrary.Conv_IntToDouble` _r_4)) _returnvalue_4))
      (bind _outactors (`GameplayStatics.GetAllActorsOfClass` "/Game/BeeKeeper/Blueprints/RestoredHive/BP_RestoredHive.BP_RestoredHive_C"))
      (for _array_element_5 _outactors
        (for _array_element_6 (`/Game/BeeKeeper/Blueprints/SaveGame/BP_SaveGame.RestoredHives` (`self.SaveData`))
          (if (`|EnumEquality` (`.BaseSpecies_13_A168E76D44BD4A04E19FBDA8B0FE6C8E` (break `/Game/BeeKeeper/Blueprints/SaveGame/S_RestoredHiveSaveData` _array_element_6)) (`/Game/BeeKeeper/Blueprints/RestoredHive/BP_RestoredHive.Species` _array_element_5))
            (`/Game/BeeKeeper/Blueprints/RestoredHive/BP_RestoredHive.LoadRestoredHiveFromSaveData` _array_element_5 _array_element_6)))))
    (:`then_1`
      (for _array_element_7 (`/Game/BeeKeeper/Blueprints/SaveGame/BP_SaveGame.BeePropsSave` (`self.SaveData`))
        (bind _returnvalue_5 (`|SpawnActorFromClass` "/Game/BeeKeeper/Gentic/Blueprints/BP_BeeProp.BP_BeeProp_C" (break `/Game/BeeKeeper/Blueprints/SaveGame/S_BeePropSaveData` _array_element_7) "Undefined" "OverrideRootScale" null true null))
        (bind (_main _sec _speed _fertility) (break `/Game/BeeKeeper/Blueprints/SaveGame/S_BeeSaveData` (`.BeeData_5_03679E30445260C3580191B03F3F8BD6` (break `/Game/BeeKeeper/Blueprints/SaveGame/S_BeePropSaveData` _array_element_7))))
        (bind _returnvalue_6 (`BeeGenetic.Construct` _main _sec _speed _fertility))
        (`/Game/BeeKeeper/Gentic/Blueprints/BP_BeeProp.UpdateBeeProps` _returnvalue_5 _returnvalue_6 "BeeProp")))
    (:`then_2`
      (`BeeGenetic.ClearDiscoveredSpecies`)
      (for _array_element_8 (`/Game/BeeKeeper/Blueprints/SaveGame/BP_SaveGame.DiscoveredSpecies` (`self.SaveData`))
        (`BeeGenetic.DiscoverSpeciesType` _array_element_8))
      (bind _values (`BlueprintMapLibrary.Map_Values` (`self.Buildings`)))
      (for _array_element_9 _values
        (bind _asbp_bee_hive (cast `/Game/BeeKeeper/BeeHive/BP_BeeHive` _array_element_9))
        (for (_array_element_10 _array_index) (`/Game/BeeKeeper/BeeHive/BP_BeeHive.Bees` _asbp_bee_hive)
          (if (!= _array_index 0)
            (`/Game/BeeKeeper/UI/WB_HexSlot.MarkNewSpecies` (`|GetArrayItem` (`/Game/BeeKeeper/UI/WB_BeeHiveStats.Slots` (`/Game/BeeKeeper/BeeHive/BP_BeeHive.Bee Hive Stats WB` _asbp_bee_hive)) _array_index) (`BeeGenetic.Main` _array_element_10) (`BeeGenetic.Sec` _array_element_10))))))))

(fn `ResearchBeehiveCapacity`
  (params (ExpectedResult :type Integer))
  (locals (ExpectedBeforeResearch :type Integer))
  (bind _expectedbeforeresearch (`local.ExpectedBeforeResearch`))
  (set `local.ExpectedBeforeResearch` (- ExpectedResult 1))
  (bind _values (`BlueprintMapLibrary.Map_Values` (`self.Buildings`)))
  (for _array_element _values
    (bind _asbp_bee_hive (cast `/Game/BeeKeeper/BeeHive/BP_BeeHive` _array_element))
    (bind _returnvalue (`KismetArrayLibrary.Array_Length` (`/Game/BeeKeeper/BeeHive/BP_BeeHive.FramesData` _asbp_bee_hive)))
    (if (== _returnvalue _expectedbeforeresearch)
      (`/Game/BeeKeeper/BeeHive/BP_BeeHive.UpgradeFramesCount` _asbp_bee_hive)
      (else
        (`KismetSystemLibrary.PrintText` (`|FormatText` "Unexpected beehive frames count state for research capacity. Expected {0} count, but have {1} count" _expectedbeforeresearch _returnvalue) true true (struct :`R` 1.0 :`A` 1.0) 10.0)))))

(fn `SetLowGraphics`
  (params (Value :type Integer))
  (bind _returnvalue (`GameUserSettings.GetGameUserSettings`))
  (`GameUserSettings.SetOverallScalabilityLevel` _returnvalue Value)
  (`GameUserSettings.ApplyNonResolutionSettings` _returnvalue))

(fn `SpeedGens`
  (`BlueprintGameplayTagLibrary.AddGameplayTag` (`/Game/BeeKeeper/Blueprints/SaveGame/BP_SaveGame.CompletedResearch` (`self.SaveData`)) (struct :`TagName` "Research.SpeedGens"))
  (bind _values (`BlueprintMapLibrary.Map_Values` (`self.Buildings`)))
  (for _array_element _values
    (bind _asbp_bee_hive (cast `/Game/BeeKeeper/BeeHive/BP_BeeHive` _array_element))
    (bind _bee_hive_stats_wb (`/Game/BeeKeeper/BeeHive/BP_BeeHive.Bee Hive Stats WB` _asbp_bee_hive))
    (if (`Widget.IsVisible` _bee_hive_stats_wb)
      (`/Game/BeeKeeper/UI/WB_BeeHiveStats.OnSlotHovered` _bee_hive_stats_wb (`/Game/BeeKeeper/UI/WB_BeeHiveStats.SelectedIndex` _bee_hive_stats_wb)))))

(fn `Stage1`
  (`|ExecutionSequence`
    (:`then_0`
      (bind _asbp_first_person_controller (cast `/Game/BeeKeeper/Blueprints/FirstPersonController/BP_FirstPersonController` (`GameplayStatics.GetPlayerCharacter` 0)))
      (`/Game/BeeKeeper/UI/WB_ResearchTree.SetEnabledStages` (`/Game/BeeKeeper/UI/WB_HandInventory.WB_ResearchTree` (`/Game/BeeKeeper/Blueprints/FirstPersonController/BP_FirstPersonController.WB_HandInventoryRef` _asbp_first_person_controller)) 1)
      (set `/Game/BeeKeeper/Blueprints/SaveGame/BP_SaveGame.RestoringStage` 1 (`self.SaveData`)))
    (:`then_1`
      (bind _returnvalue (`GameplayStatics.GetActorOfClass` "/Game/BeeKeeper/Blueprints/BeeAltar/BP_BeeAltar.BP_BeeAltar_C"))
      (`/Game/BeeKeeper/Blueprints/BeeAltar/BP_BeeAltar.ChangeStage` _returnvalue 1))))

(fn `Stage2`
  (`|ExecutionSequence`
    (:`then_0`
      (bind _asbp_first_person_controller (cast `/Game/BeeKeeper/Blueprints/FirstPersonController/BP_FirstPersonController` (`GameplayStatics.GetPlayerCharacter` 0)))
      (`/Game/BeeKeeper/UI/WB_ResearchTree.SetEnabledStages` (`/Game/BeeKeeper/UI/WB_HandInventory.WB_ResearchTree` (`/Game/BeeKeeper/Blueprints/FirstPersonController/BP_FirstPersonController.WB_HandInventoryRef` _asbp_first_person_controller)) 2)
      (set `/Game/BeeKeeper/Blueprints/SaveGame/BP_SaveGame.RestoringStage` 2 (`self.SaveData`)))
    (:`then_1`
      (bind _returnvalue (`GameplayStatics.GetActorOfClass` "/Game/BeeKeeper/Blueprints/BeeAltar/BP_BeeAltar.BP_BeeAltar_C"))
      (`/Game/BeeKeeper/Blueprints/BeeAltar/BP_BeeAltar.ChangeStage` _returnvalue 2))))

(fn `Stage3`
  (`|ExecutionSequence`
    (:`then_0`
      (bind _asbp_first_person_controller (cast `/Game/BeeKeeper/Blueprints/FirstPersonController/BP_FirstPersonController` (`GameplayStatics.GetPlayerCharacter` 0)))
      (`/Game/BeeKeeper/UI/WB_ResearchTree.SetEnabledStages` (`/Game/BeeKeeper/UI/WB_HandInventory.WB_ResearchTree` (`/Game/BeeKeeper/Blueprints/FirstPersonController/BP_FirstPersonController.WB_HandInventoryRef` _asbp_first_person_controller)) 3)
      (set `/Game/BeeKeeper/Blueprints/SaveGame/BP_SaveGame.RestoringStage` 3 (`self.SaveData`)))
    (:`then_1`
      (bind _returnvalue (`GameplayStatics.GetActorOfClass` "/Game/BeeKeeper/Blueprints/BeeAltar/BP_BeeAltar.BP_BeeAltar_C"))
      (`/Game/BeeKeeper/Blueprints/BeeAltar/BP_BeeAltar.ChangeStage` _returnvalue 3))))

(fn `Stage4`
  (`|ExecutionSequence`
    (:`then_0`
      (bind _asbp_first_person_controller (cast `/Game/BeeKeeper/Blueprints/FirstPersonController/BP_FirstPersonController` (`GameplayStatics.GetPlayerCharacter` 0)))
      (`/Game/BeeKeeper/UI/WB_ResearchTree.SetEnabledStages` (`/Game/BeeKeeper/UI/WB_HandInventory.WB_ResearchTree` (`/Game/BeeKeeper/Blueprints/FirstPersonController/BP_FirstPersonController.WB_HandInventoryRef` _asbp_first_person_controller)) 4)
      (set `/Game/BeeKeeper/Blueprints/SaveGame/BP_SaveGame.RestoringStage` 4 (`self.SaveData`)))
    (:`then_1`
      (bind _returnvalue (`GameplayStatics.GetActorOfClass` "/Game/BeeKeeper/Blueprints/BeeAltar/BP_BeeAltar.BP_BeeAltar_C"))
      (`/Game/BeeKeeper/Blueprints/BeeAltar/BP_BeeAltar.ChangeStage` _returnvalue 4))))

(fn `Update Discovered Bees`
  (params (Bee :type "BeeGenetic Object Reference"))
  (bind _sec (`BeeGenetic.Sec` Bee))
  (bind _returnvalue (`BeeGenetic.IsDiscoveredSpecies` (`BeeGenetic.Main` Bee)))
  (if (not _returnvalue)
    (`BeeGenetic.DiscoverSpecies` Bee)
    (bind _values (`BlueprintMapLibrary.Map_Values` (`self.Buildings`) :!label _label))
    (for _array_element _values
      (bind _asbp_bee_hive (cast `/Game/BeeKeeper/BeeHive/BP_BeeHive` _array_element))
      (for (_array_element_2 _array_index) (`/Game/BeeKeeper/BeeHive/BP_BeeHive.Bees` _asbp_bee_hive)
        (`/Game/BeeKeeper/UI/WB_HexSlot.MarkNewSpecies` (`|GetArrayItem` (`/Game/BeeKeeper/UI/WB_BeeHiveStats.Slots` (`/Game/BeeKeeper/BeeHive/BP_BeeHive.Bee Hive Stats WB` _asbp_bee_hive)) _array_index) (`BeeGenetic.Main` _array_element_2) (`BeeGenetic.Sec` _array_element_2))))
    (else
      (bind _returnvalue_2 (`BeeGenetic.IsDiscoveredSpecies` _sec))
      (if (not _returnvalue_2)
        (`BeeGenetic.DiscoverSpeciesType` _sec)
        (goto _label)))))