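; Game mode for the bee game that spawns either the VR or the desktop player at BeginPlay.
; It picks VRPawn at VRStart when -vr is passed or an HMD is enabled, unless -novr is present; otherwise it spawns BP_FirstPersonController at DesktopStart.
; An unconnected "Bees Pentagram" graph, which never runs, would attach a pentagram of non-colliding bee props to the desktop camera.
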(event `self.ReceiveBeginPlay`
  (bind _returnvalue (`KismetSystemLibrary.GetCommandLine`))
  (if (and (or (`KismetStringLibrary.Contains` _returnvalue "-vr") (`HeadMountedDisplayFunctionLibrary.IsHeadMountedDisplayEnabled`)) (not (`KismetStringLibrary.Contains` _returnvalue "-novr")))
    (`|SpawnActorFromClass` "/Game/VRTemplate/Blueprints/VRPawn.VRPawn_C" (`self.GetTransform` (`self.K2_FindPlayerStart` null "VRStart")) "Undefined" "OverrideRootScale" null null)
    (else
      (bind _returnvalue_2 (`|SpawnActorFromClass` "/Game/BeeKeeper/Blueprints/FirstPersonController/BP_FirstPersonController.BP_FirstPersonController_C" (`self.GetTransform` (`self.K2_FindPlayerStart` null "DesktopStart")) "Undefined" "OverrideRootScale" null null)))))

(fn `UserConstructionScript`)