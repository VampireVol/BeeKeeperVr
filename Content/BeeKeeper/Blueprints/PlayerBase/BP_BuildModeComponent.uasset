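; Player build-mode component for placing, rotating and demolishing beehives on a hex grid.
; While active, it ticks, tracing from a source component, snapping to hex centres and tagged floor, and moving a spawned grid and preview hive there.
; Overlap checks tint the placement ghost as buildable or blocked; destroy mode overlays a highlight on the targeted hive.
; Confirming spawns or destroys hives, updating the game instance's map keyed by hex coordinates.
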(event `self.ReceiveBeginPlay`
  (bind _returnvalue (`|SpawnActorFromClass` "/Game/BeeKeeper/Blueprints/PlayerBase/BP_BuildGrid.BP_BuildGrid_C" (`Actor.GetTransform` (`GameplayStatics.GetPlayerController` 0)) "Undefined" "OverrideRootScale" null null))
  (`SceneComponent.K2_AddWorldOffset` (`/Game/BeeKeeper/Blueprints/PlayerBase/BP_BuildGrid.DefaultSceneRoot` _returnvalue) (0.0 0.0 5.0) false false)
  (bind _output_get (set `self.BuildGridRef` _returnvalue))
  (set `self.BuildGrid` (`/Game/BeeKeeper/Blueprints/PlayerBase/BP_BuildGrid.BuildGrid` _output_get))
  (bind _asbp_bee_game_instance (cast `/Game/BeeKeeper/Blueprints/BP_BeeGameInstance` (`GameplayStatics.GetGameInstance`))
    (:`then`
      (set `self.GameInstance` _asbp_bee_game_instance))
    (:`CastFailed`
      (`KismetSystemLibrary.PrintText` "Can't init correct game instance"))))

(event `self.ReceiveTick`
  (params (DeltaSeconds :type "Float (single-precision)"))
  ;[1 1 1] Actuialy tick disabled when build mode disable
  (if (`self.BuildModeEnabled`)
    (bind (_hitposition _hitactor) (`self.TraceFromSource`))
    (bind _position (`self.TryGetFloorPosition` _hitposition))
    (`self.DrawDebugHexCell` _position)
    (`SceneComponent.K2_SetWorldLocation` (`self.BuildGrid`) (+ _position (0.0 0.0 1.0)) false false)
    (if (not (`self.DestroyModeEnabled`))
      (`self.PlaceBeeHive` _position)
      (`self.SetBeeHiveBuildMat`)
      (else
        (`self.PlaceBeeHiveForDestroy` _position _hitactor)))))

(fn `BuildActionProcess`
  (bind (_returnvalue_location _returnvalue_rotation) (`KismetMathLibrary.BreakTransform` (`Actor.GetTransform` (`self.BeeHiveForPlace`))))
  (if (`self.BuildModeEnabled`)
    (if (`self.DestroyModeEnabled`)
      (bind _beehivefordestroy (`self.BeeHiveForDestroy`)
        (:`then`
          (bind (_returnvalue_x _returnvalue_y) (`KismetMathLibrary.BreakVector` (`Actor.K2_GetActorLocation` _beehivefordestroy)))
          (bind (_q _r) (`/Game/BeeKeeper/BeeHive/BP_GridLibrary.PixelToHex` _returnvalue_x _returnvalue_y))
          (bind _returnvalue (`KismetMathLibrary.Conv_IntToDouble` _q))
          (bind _returnvalue_2 (`KismetMathLibrary.Conv_IntToDouble` _r))
          (bind (_value _returnvalue_3) (`BlueprintMapLibrary.Map_Find` (`/Game/BeeKeeper/Blueprints/BP_BeeGameInstance.BeeHives` (`self.GameInstance`)) (`KismetMathLibrary.MakeVector2D` _returnvalue _returnvalue_2)))
          (if _returnvalue_3
            (`Actor.K2_DestroyActor` _value)
            (`BlueprintMapLibrary.Map_Remove` (`/Game/BeeKeeper/Blueprints/BP_BeeGameInstance.BeeHives` (`self.GameInstance`)) (`KismetMathLibrary.MakeVector2D` _returnvalue _returnvalue_2))))
        (:`else`))
      (elif (`self.CanBuild`)
        (bind _returnvalue_4 (`|SpawnActorFromClass` "/Game/BeeKeeper/BeeHive/BP_BeeHive.BP_BeeHive_C" (`KismetMathLibrary.MakeTransform` _returnvalue_location _returnvalue_rotation) "Undefined" "OverrideRootScale" null true null))
        (`Actor.K2_DestroyActor` (`self.BeeHiveForPlace`))
        (set `self.BeeHiveForPlace` null)
        (bind (_returnvalue_x_2 _returnvalue_y_2) (`KismetMathLibrary.BreakVector` (`Actor.K2_GetActorLocation` _returnvalue_4)))
        (bind (_q_2 _r_2) (`/Game/BeeKeeper/BeeHive/BP_GridLibrary.PixelToHex` _returnvalue_x_2 _returnvalue_y_2))
        (`BlueprintMapLibrary.Map_Add` (`/Game/BeeKeeper/Blueprints/BP_BeeGameInstance.BeeHives` (`self.GameInstance`)) (`KismetMathLibrary.MakeVector2D` (`KismetMathLibrary.Conv_IntToDouble` _q_2) (`KismetMathLibrary.Conv_IntToDouble` _r_2)) _returnvalue_4)))))

(fn `Disable Bee Hive Collision Spheres `
  (params (BeeHive :type "/Game/BeeKeeper/BeeHive/BP_BeeHive Object Reference"))
  (`PrimitiveComponent.SetCollisionResponseToAllChannels` (`/Game/BeeKeeper/BeeHive/BP_BeeHive.BeeSphereLeft` BeeHive) "ECR_Ignore")
  (`PrimitiveComponent.SetCollisionResponseToAllChannels` (`/Game/BeeKeeper/BeeHive/BP_BeeHive.BeeSphereRight` BeeHive) "ECR_Ignore"))

(fn `DrawDebugHexCell`
  (params (CenterPos :type "Vector Structure"))
  (if (`self.IsDrawDebugCell`)
    (for _index (range 6)
      (bind (_x _y) (`/Game/BeeKeeper/BeeHive/BP_GridLibrary.FlatHexCorner` CenterPos_X CenterPos_Y _index))
      (`KismetSystemLibrary.DrawDebugLine` (`KismetMathLibrary.MakeVector` _x _y CenterPos_Z) (`KismetMathLibrary.MakeVector` _x _y (+ CenterPos_Z 200.0)) (struct :`R` 1.0 :`A` 1.0) 0.5 1.0))))

(fn `PlaceBeeHive`
  (params (BeeHiveLocation :type "Vector Structure"))
  (bind _beehiveforplace (`self.BeeHiveForPlace`))
  (`self.BeeHiveForPlace`
    (:`then`
      (`Actor.K2_SetActorLocationAndRotation` (`self.BeeHiveForPlace`) BeeHiveLocation (`self.BuildingRotator`) false false))
    (:`else`
      (bind _returnvalue (`|SpawnActorFromClass` "/Game/BeeKeeper/BeeHive/BP_BeeHive.BP_BeeHive_C" (`KismetMathLibrary.MakeTransform` BeeHiveLocation (`self.BuildingRotator`) (0.99 0.99 0.99)) "Undefined" "OverrideRootScale" null true null))
      (set `self.BeeHiveForPlace` _returnvalue)
      (`PrimitiveComponent.SetCollisionResponseToChannel` (`/Game/BeeKeeper/BeeHive/BP_BeeHive.Beehive` (`self.BeeHiveForPlace`)) "ECC_PhysicsBody" "ECR_Ignore")
      (`PrimitiveComponent.SetCollisionResponseToChannel` (`/Game/BeeKeeper/BeeHive/BP_BeeHive.Beehive` _beehiveforplace) "ECC_Pawn" "ECR_Ignore")
      (for _array_element (`Actor.GetAttachedActors` _beehiveforplace true false)
        (bind _returnvalue_2 (`Actor.GetComponentByClass` _array_element "/Script/Engine.StaticMeshComponent"))
        (`PrimitiveComponent.SetCollisionResponseToChannel` _returnvalue_2 "ECC_PhysicsBody" "ECR_Ignore")
        (`PrimitiveComponent.SetCollisionResponseToChannel` _returnvalue_2 "ECC_Pawn" "ECR_Ignore")))))

(fn `PlaceBeeHiveForDestroy`
  (params (BeeHivePostion :type "Vector Structure") (HitActor :type "Actor Object Reference"))
  (bind _beehivefordestroy (`self.BeeHiveForDestroy`))
  (bind _cannotbuildmat (`self.CanNotBuildMat`))
  (`/Engine/EditorBlueprintResources/StandardMacros.IsValid` HitActor
    (:`Is Valid`
      (bind _asbp_bee_hive (cast `/Game/BeeKeeper/BeeHive/BP_BeeHive` HitActor)
        (:`then`
          (bind _beehivefordestroy_2 (`self.BeeHiveForDestroy`)
            (:`then`
              (bind _returnvalue (`Actor.K2_GetActorRotation` _asbp_bee_hive))
              (`Actor.K2_SetActorLocationAndRotation` _beehivefordestroy_2 BeeHivePostion _returnvalue false false))
            (:`else`
              (bind _returnvalue_2 (`|SpawnActorFromClass` "/Game/BeeKeeper/BeeHive/BP_BeeHive.BP_BeeHive_C" (`KismetMathLibrary.MakeTransform` BeeHivePostion _returnvalue (1.01 1.01 1.01)) "Undefined" "OverrideRootScale" null true null))
              (set `self.BeeHiveForDestroy` _returnvalue_2)
              (`PrimitiveComponent.SetCollisionResponseToChannel` (`/Game/BeeKeeper/BeeHive/BP_BeeHive.Beehive` (`self.BeeHiveForDestroy`)) "ECC_PhysicsBody" "ECR_Ignore")
              (`PrimitiveComponent.SetCollisionResponseToChannel` (`/Game/BeeKeeper/BeeHive/BP_BeeHive.Beehive` (`self.BeeHiveForDestroy`)) "ECC_Pawn" "ECR_Ignore")
              (for _array_element (`Actor.K2_GetComponentsByClass` _beehivefordestroy "/Script/Engine.MeshComponent")
                (for (_ _array_index) (`MeshComponent.GetMaterials` _array_element)
                  (`PrimitiveComponent.SetMaterial` _array_element _array_index _cannotbuildmat)))
              (for _array_element_2 (`Actor.GetAttachedActors` _beehivefordestroy true false)
                (for _array_element_3 (`Actor.K2_GetComponentsByClass` _array_element_2 "/Script/Engine.MeshComponent")
                  (for (_ _array_index_2) (`MeshComponent.GetMaterials` _array_element_3)
                    (`PrimitiveComponent.SetMaterial` _array_element_3 _array_index_2 _cannotbuildmat)))))))
        (:`CastFailed`
          (bind _beehivefordestroy_3 (`self.BeeHiveForDestroy` :!label _label)
            (:`then`
              (`Actor.K2_DestroyActor` _beehivefordestroy_3)
              (set `self.BeeHiveForDestroy` null))
            (:`else`)))))
    (:`Is Not Valid`
      (goto _label))))

(fn `RotateBeeHive`
  (params (IsRotateRight :type Boolean))
  (locals (RotatorRight :type "Rotator Structure" :default (struct :`Yaw` 60.0)) (RotatorLeft :type "Rotator Structure" :default (struct :`Yaw` -60.0)))
  (set `self.BuildingRotator` (`KismetMathLibrary.ComposeRotators` (`self.BuildingRotator`) (select `bool` IsRotateRight :`false` (`local.RotatorRight`) :`true` (`local.RotatorLeft`)))))

(fn `SetBeeHiveBuildMat`
  (locals (FloorChecked :type Boolean) (OverlappingCount :type Integer))
  (bind _beehiveforplace (`self.BeeHiveForPlace`))
  (bind _beehiveforplace_2 (`self.BeeHiveForPlace`))
  (bind _overlappingactors (`Actor.GetOverlappingActors` _beehiveforplace_2 null))
  (bind _returnvalue (select `bool` (`self.CanBuild`) :`false` (`self.CanNotBuildMat`) :`true` (`self.CanBuildMat`)))
  (set `local.OverlappingCount` (`KismetArrayLibrary.Array_Length` _overlappingactors))
  (for _array_element _overlappingactors
    (if (`Actor.ActorHasTag` _array_element "IsFloor")
      (set `local.FloorChecked` true)
      (set `local.OverlappingCount` (- (`local.OverlappingCount`) 1) :!label _label)
      (elif (`KismetArrayLibrary.Array_Contains` (`Actor.GetAttachedActors` _beehiveforplace_2 true false) _array_element)
        (goto _label))))
  (set `self.CanBuild` (not (or (not (`local.FloorChecked`)) (> (`local.OverlappingCount`) 0))))
  (for _array_element_2 (`Actor.K2_GetComponentsByClass` _beehiveforplace "/Script/Engine.MeshComponent")
    (for (_ _array_index) (`MeshComponent.GetMaterials` _array_element_2)
      (`PrimitiveComponent.SetMaterial` _array_element_2 _array_index _returnvalue)))
  (for _array_element_3 (`Actor.GetAttachedActors` _beehiveforplace true false)
    (for _array_element_4 (`Actor.K2_GetComponentsByClass` _array_element_3 "/Script/Engine.MeshComponent")
      (for (_ _array_index_2) (`MeshComponent.GetMaterials` _array_element_4)
        (`PrimitiveComponent.SetMaterial` _array_element_4 _array_index_2 _returnvalue)))))

(fn `SetBuildTraceSource`
  (params (BuildTraceSource :type "SceneComponent Object Reference"))
  (set `self.BuildTraceSource` BuildTraceSource))

(fn `SwitchBuildMode`
  (params (IsBuildModeEnabled :type Boolean))
  (bind _output_get (set `self.BuildModeEnabled` IsBuildModeEnabled))
  (`SceneComponent.SetVisibility` (`self.BuildGrid`) _output_get false)
  (`self.SetComponentTickEnabled` _output_get)
  (`|ExecutionSequence`
    (:`then_0`
      (bind _beehiveforplace (`self.BeeHiveForPlace`)
        (:`then`
          (`Actor.K2_DestroyActor` _beehiveforplace)
          (set `self.BeeHiveForPlace` null))
        (:`else`)))
    (:`then_1`
      (bind _beehivefordestroy (`self.BeeHiveForDestroy`)
        (:`then`
          (`Actor.K2_DestroyActor` _beehivefordestroy)
          (set `self.BeeHiveForDestroy` null))
        (:`else`)))
    (:`then_2`
      (set `self.DestroyModeEnabled` false))))

(fn `SwitchDestroyMode`
  (if (`self.BuildModeEnabled`)
    (set `self.DestroyModeEnabled` (not (`self.DestroyModeEnabled`)))
    (bind _beehiveforplace (`self.BeeHiveForPlace`)
      (:`then`
        (`Actor.K2_DestroyActor` _beehiveforplace))
      (:`else`
        _))
    (bind _beehivefordestroy (`self.BeeHiveForDestroy`)
      (:`then`
        (`Actor.K2_DestroyActor` _beehivefordestroy))
      (:`else`))))

(fn `TraceFromSource`
  (returns (HitPosition :type "Vector Structure") (HitActor :type "Actor Object Reference"))
  (bind _buildtracesource (`self.BuildTraceSource`))
  (bind _returnvalue (`SceneComponent.K2_GetComponentLocation` _buildtracesource))
  (bind (_outhit _returnvalue_2) (`KismetSystemLibrary.LineTraceSingle` _returnvalue (+ _returnvalue (* (`SceneComponent.GetForwardVector` _buildtracesource) 1000.0)) "TraceTypeQuery1" false (`|MakeArray` (`self.BeeHiveForPlace`) (`self.BeeHiveForDestroy`) :!type "Actor Object Reference")))
  (bind (_bblockinghit _binitialoverlap _time _distance _location _impactpoint _normal _impactnormal _physmat _hitactor _hitcomponent _hitbonename _bonename _hititem _elementindex _faceindex _tracestart _traceend) (`GameplayStatics.BreakHitResult` _outhit))
  (bind (_centerx _centery) (`/Game/BeeKeeper/BeeHive/BP_GridLibrary.GetCenterHex` (.x (select `bool` _returnvalue_2 :`false` _traceend :`true` _location)) (.y (select `bool` _returnvalue_2 :`false` _traceend :`true` _location))))
  (return (`KismetMathLibrary.MakeVector` _centerx _centery (.z (select `bool` _returnvalue_2 :`false` _traceend :`true` _location))) _hitactor))

(fn `TryGetFloorPosition`
  (params (StartPos :type "Vector Structure"))
  (returns (Position :type "Vector Structure"))
  (locals (LocalPos :type "Vector Structure") (FloorChecked :type Boolean) (Ignore :type "Array of /Game/BeeKeeper/BeeHive/BP_BeeHive Object Reference"))
  (bind _asbp_bee_game_instance (cast `/Game/BeeKeeper/Blueprints/BP_BeeGameInstance` (`GameplayStatics.GetGameInstance`)))
  (bind _values (`BlueprintMapLibrary.Map_Values` (`/Game/BeeKeeper/Blueprints/BP_BeeGameInstance.BeeHives` _asbp_bee_game_instance)))
  (bind _output_get (set `local.Ignore` _values))
  (`KismetArrayLibrary.Array_Add` _output_get (`self.BeeHiveForPlace`))
  (`KismetArrayLibrary.Array_Add` _output_get (`self.BeeHiveForDestroy`))
  (bind _outhits (`KismetSystemLibrary.LineTraceMulti` StartPos (- StartPos (0.0 0.0 300.0)) "TraceTypeQuery4" false (`local.Ignore`) "ForDuration"))
  (for _array_element _outhits
    (bind (_bblockinghit _binitialoverlap _time _distance _location _impactpoint _normal _impactnormal _physmat _hitactor) (`GameplayStatics.BreakHitResult` _array_element))
    (if (`Actor.ActorHasTag` _hitactor "IsFloor")
      (set `local.LocalPos` _location)
      (set `local.FloorChecked` true)
      (break)))
  (return (select `bool` (and (`KismetArrayLibrary.Array_IsNotEmpty` _outhits) (`local.FloorChecked`)) :`false` StartPos :`true` (`local.LocalPos`))))