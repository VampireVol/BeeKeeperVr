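; Resource producer component that turns the honeycombs in bee frames into produced items.
; ProduceFromFrames feeds each frame's honeycombs into a per-comb-type Accumulator using DT_CombRecipes, then converts that into the ItemsOutput map.
; The accumulation and conversion are delegated to AccumulateCombs and ProduceItemsFromCombs, with both maps printed on screen afterwards for debugging.
; Disconnected nodes hold unused inline production logic, including random-range yields.
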(fn `PrintDebugAccumulator`
  (bind _accumulator (`self.Accumulator`))
  (bind _values (`BlueprintMapLibrary.Map_Values` _accumulator))
  (bind _keys (`BlueprintMapLibrary.Map_Keys` _accumulator))
  (for (_array_element _array_index) _keys
    (`KismetSystemLibrary.PrintText` (`|FormatText` "Comb type: {0} Values:" (`|GetEnumeratorNameAsString` _array_element)) true true (struct :`G` 0.66 :`B` 1.0 :`A` 1.0) 10.0)
    (for _array_element_2 (`.Items` (break `AccumulatorComb` (`|GetArrayItem` _values _array_index)))
      (bind (_itemtype _amount _cost _remainingcount) (break `AccumulatorCombItem` _array_element_2))
      (`KismetSystemLibrary.PrintText` (`|FormatText` "Item type: {0} Amount: {1} Cost {2} Count {3}" (`|GetEnumeratorNameAsString` _itemtype) _amount _cost _remainingcount) true true (struct :`G` 0.66 :`B` 1.0 :`A` 1.0) 10.0))))

(fn `PrintDebugProduced`
  (bind _itemsoutput (`self.ItemsOutput`))
  (bind _values (`BlueprintMapLibrary.Map_Values` _itemsoutput))
  (bind _keys (`BlueprintMapLibrary.Map_Keys` _itemsoutput))
  (for (_array_element _array_index) _keys
    (`KismetSystemLibrary.PrintText` (`|FormatText` "Produced: {1} {2}" (`|GetArrayItem` _values _array_index) (`|GetEnumeratorNameAsString` _array_element)) true true (struct :`G` 0.66 :`B` 1.0 :`A` 1.0) 10.0)))

(fn `ProduceFromFrames`
  (params (Frames :type "Array of /Game/BeeKeeper/Blueprints/Inventory/S_FrameData Structure"))
  (locals (FrameCapacity :type Integer :default 100))
  (for _array_element Frames
    (`BeeFunctionLibrary.AccumulateCombs` (`.Honeycombs_11_CF7265A945E098E2D0E51F8BAF63BA69` (break `/Game/BeeKeeper/Blueprints/Inventory/S_FrameData` _array_element)) (`self.Accumulator`) "/Game/BeeKeeper/Blueprints/ResourceProducer/DT_CombRecipes.DT_CombRecipes"))
  (`BeeFunctionLibrary.ProduceItemsFromCombs` (`self.Accumulator`) (`self.ItemsOutput`) "/Game/BeeKeeper/Blueprints/ResourceProducer/DT_CombRecipes.DT_CombRecipes")
  (`self.PrintDebugProduced`)
  (`self.PrintDebugAccumulator`))