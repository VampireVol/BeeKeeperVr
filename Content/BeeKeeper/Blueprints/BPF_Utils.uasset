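; BPF_Utils is a stateless helper library for the BeeKeeper game, covering hive frames, bees, item slots, icons and colors.
; Frame helpers derive progress by summing honeycomb values over 100, and reset frames by clearing honeycombs, snapshots and tags, with seed regeneration still a TODO.
; Other helpers convert bees to save data, check slot occupancy, scale color channels by 256, and build icon brushes from DT_ItemsData with a Star fallback.
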(fn `CalcFrameProgress`
  (params (S_FrameData :type "/Game/BeeKeeper/Blueprints/Inventory/S_FrameData Structure (by ref)"))
  (returns (ReturnValue :type "Float (double-precision)"))
  (locals (Sum :type Integer))
  (bind _values (`BlueprintMapLibrary.Map_Values` (`.Honeycombs_11_CF7265A945E098E2D0E51F8BAF63BA69` (break `/Game/BeeKeeper/Blueprints/Inventory/S_FrameData` S_FrameData))))
  (for _array_element _values
    (set `local.Sum` (+ _array_element (`local.Sum`))))
  (return (/ (`local.Sum`) 100)))

(fn `ClearFrameData`
  (params (Frame :type "/Game/BeeKeeper/Blueprints/Inventory/S_FrameData Structure (by ref)"))
  (bind (_honeycombs _snapshots _tags) (break `/Game/BeeKeeper/Blueprints/Inventory/S_FrameData` Frame))
  (`BlueprintMapLibrary.Map_Clear` _honeycombs)
  (`KismetArrayLibrary.Array_Clear` _snapshots)
  (bind (_arrayindex _arrayelement) (`/Engine/EditorBlueprintResources/StandardMacros.ReverseForEachLoop` (`BlueprintGameplayTagLibrary.BreakGameplayTagContainer` _tags))
    (:`LoopBody`
      (`BlueprintGameplayTagLibrary.RemoveGameplayTag` _tags _arrayelement))))

(fn `FromColorToLinear`
  (params (Color :type "Color Structure (by ref)"))
  (returns (NewParam :type "LinearColor Structure"))
  (bind (_b _g _r _a) (break `Color` Color))
  (return (make `LinearColor` (/ _r 256.0) (/ _g 256.0) (/ _b 256.0) (/ _a 256.0))))

(fn `GetBeesDataFromBees`
  (params (Bees :type "Array of BeeGenetic Object Reference"))
  (returns (BeesData :type "Array of /Game/BeeKeeper/Blueprints/SaveGame/S_BeeSaveData Structure"))
  (locals (BeesOut :type "Array of /Game/BeeKeeper/Blueprints/SaveGame/S_BeeSaveData Structure"))
  (for _array_element Bees
    (`KismetArrayLibrary.Array_Add` (`local.BeesOut`) (make `/Game/BeeKeeper/Blueprints/SaveGame/S_BeeSaveData` (`BeeGenetic.Main` _array_element) (`BeeGenetic.Sec` _array_element) (`BeeGenetic.Speed` _array_element) (`BeeGenetic.Fertility` _array_element))))
  (return (`local.BeesOut`)))

(fn `GetItemIconBrush`
  (params (ItemType :type "EItemType Enum" :default "None") (Width :type Integer :default 128) (Height :type Integer :default 128))
  (returns (Icon :type "SlateBrush Structure"))
  (bind _returnvalue (`self.GetItemIconTexture` ItemType))
  (return (`WidgetBlueprintLibrary.MakeBrushFromTexture` _returnvalue Width Height)))

(fn `GetItemIconTexture`
  (params (ItemType :type "EItemType Enum" :default "None"))
  (returns (ReturnValue :type "Texture2D Object Reference"))
  (bind _returnvalue (`BeeFunctionLibrary.GetItemIcon` "/Game/BeeKeeper/Blueprints/Items/DT_ItemsData.DT_ItemsData" ItemType "/Game/BeeKeeper/UI/Icons/Star.Star"))
  (return _returnvalue))

(fn `Has Slot Item`
  (params (data :type "/Game/BeeKeeper/Blueprints/Inventory/S_SlotData Structure"))
  (returns (HasItem :type Boolean))
  (return (!= (`.InventoryIdx_5_579F21AC4D8636E5B62930970C700287` (break `/Game/BeeKeeper/Blueprints/Inventory/S_SlotData` data)) -1)))