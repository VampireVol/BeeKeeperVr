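; Restored hive actor that keeps up to three BP_BeeProp bees of its species spawned around it.
; A looping timer spawns each bee at whichever of three spawn points is farthest from existing bees, with genetics from RestoredBeesSubsystem.
; Destroyed bees leave the tracked list and restart spawning.
; Save and load functions handle bee transforms and movement state, resuming the timer through a negative initial delay.
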(event `StartSpawnBees`
  (params (InitialStartDelay :type "Float (single-precision)"))
  (if (`KismetSystemLibrary.K2_IsValidTimerHandle` (`self.SpawnTimerHandle`))
    (if (not (`KismetSystemLibrary.K2_IsTimerActiveHandle` (`self.SpawnTimerHandle`)))
      (`KismetSystemLibrary.K2_UnPauseTimerHandle` (`self.SpawnTimerHandle`)))
    (else
      (bind _returnvalue (`KismetSystemLibrary.K2_SetTimerDelegate` (delegate `SpawnBeeByTimer`) 3.0 true false InitialStartDelay))
      (set `self.SpawnTimerHandle` _returnvalue))))

(event `SpawnBeeByTimer`
  (if (< (`KismetArrayLibrary.Array_Length` (`self.SpawnedBees`)) 3)
    (bind _idx (`self.SelectSpawnPoint`))
    (`self.SpawnBee` (`KismetMathLibrary.MakeTransform` (`|GetArrayItem` (`self.SpawnPoints`) _idx) (`|GetArrayItem` (`self.SpawnRotate`) _idx)))
    (if (not (< (`KismetArrayLibrary.Array_Length` (`self.SpawnedBees`)) 3))
      (`KismetSystemLibrary.K2_ClearAndInvalidateTimerHandle` (`self.SpawnTimerHandle`)))
    (else
      (`KismetSystemLibrary.K2_PauseTimerHandle` (`self.SpawnTimerHandle`)))))

(event `BeeDestroyed` :!signature `self.OnDestroyed`
  (params (DestroyedActor :type "Actor Object Reference"))
  (bind _idx (`self.FindSpawnedBee` DestroyedActor))
  (`KismetArrayLibrary.Array_Remove` (`self.SpawnedBees`) _idx)
  (`self.StartSpawnBees` 0.0))

(event `self.ReceiveBeginPlay`
  (bind (_returnvalue_location _returnvalue_rotation) (`KismetMathLibrary.BreakTransform` (`SceneComponent.K2_GetComponentToWorld` (`self.SpawnPoint2`))))
  (bind (_returnvalue_location_2 _returnvalue_rotation_2) (`KismetMathLibrary.BreakTransform` (`SceneComponent.K2_GetComponentToWorld` (`self.SpawnPoint`))))
  (bind (_returnvalue_location_3 _returnvalue_rotation_3) (`KismetMathLibrary.BreakTransform` (`SceneComponent.K2_GetComponentToWorld` (`self.SpawnPoint1`))))
  (`KismetArrayLibrary.Array_Add` (`self.SpawnPoints`) _returnvalue_location_2)
  (`KismetArrayLibrary.Array_Add` (`self.SpawnPoints`) _returnvalue_location_3)
  (`KismetArrayLibrary.Array_Add` (`self.SpawnPoints`) _returnvalue_location)
  (`KismetArrayLibrary.Array_Add` (`self.SpawnRotate`) _returnvalue_rotation_2)
  (`KismetArrayLibrary.Array_Add` (`self.SpawnRotate`) _returnvalue_rotation_3)
  (`KismetArrayLibrary.Array_Add` (`self.SpawnRotate`) _returnvalue_rotation)
  (`self.StartSpawnBees` 0.0))

(fn `CreateBeeGenetic`
  (returns (ReturnValue :type "BeeGenetic Object Reference"))
  (bind _returnvalue (`RestoredBeesSubsystem.GetBee` (subsystem `RestoredBeesSubsystem`) (`self.Species`)))
  (return _returnvalue))

(fn `FindSpawnedBee`
  (params (Bee :type "Actor Object Reference"))
  (returns (Idx :type Integer))
  (for (_array_element _array_index) (`self.SpawnedBees`)
    (if (== _array_element Bee)
      (return _array_index)))
  (return -1))

(fn `GetRestoredHiveSaveData`
  (returns (Save :type "/Game/BeeKeeper/Blueprints/SaveGame/S_RestoredHiveSaveData Structure"))
  (locals (Bees :type "Array of Transform Structure") (NextPost :type "Array of Vector Structure") (Vel :type "Array of Vector Structure"))
  (for _array_element (`self.SpawnedBees`)
    (`KismetArrayLibrary.Array_Add` (`local.Bees`) (`self.GetTransform` _array_element))
    (`KismetArrayLibrary.Array_Add` (`local.NextPost`) (`/Game/BeeKeeper/Gentic/Blueprints/BP_BeeProp.NextPosPoint` _array_element))
    (`KismetArrayLibrary.Array_Add` (`local.Vel`) (`/Game/BeeKeeper/Gentic/Blueprints/BP_BeeProp.Velocity` _array_element)))
  (return (make `/Game/BeeKeeper/Blueprints/SaveGame/S_RestoredHiveSaveData` (`local.Bees`) (`local.NextPost`) (`local.Vel`) (`KismetSystemLibrary.K2_GetTimerElapsedTimeHandle` (`self.SpawnTimerHandle`)) (`self.Species`))))

(fn `LoadRestoredHiveFromSaveData`
  (params (Save :type "/Game/BeeKeeper/Blueprints/SaveGame/S_RestoredHiveSaveData Structure"))
  (for (_array_element _array_index) Save_Bees_3_CF952B7A496FE50C480D2991CD34A646
    (`self.SpawnBee` _array_element true)
    (`/Game/BeeKeeper/Gentic/Blueprints/BP_BeeProp.LoadSimFromSaveData` (`|GetArrayItem` (`self.SpawnedBees`) _array_index) (`|GetArrayItem` Save_BeeVel_19_3FC7E8944C05174DAEDF0982E627A9B3 _array_index) (`|GetArrayItem` Save_NextBeePos_17_F85298D54FEE5B43E5946F83678F1642 _array_index)))
  (`KismetSystemLibrary.K2_ClearAndInvalidateTimerHandle` (`self.SpawnTimerHandle`))
  (`self.StartSpawnBees` (* Save_TimerTime_10_A4F0241B487AA066349B2FB9C402F854 -1.0)))

(fn `SelectSpawnPoint`
  (returns (Idx :type Integer))
  (locals (MinIdx :type Integer) (NearestBee :type "Float (double-precision)") (DistantBee :type "Float (double-precision)"))
  (for (_array_element _array_index) (`self.SpawnPoints`)
    (set `local.NearestBee` 100000.0)
    (for _array_element_2 (`self.SpawnedBees`)
      (set `local.NearestBee` (`KismetMathLibrary.FMin` (`local.NearestBee`) (`KismetMathLibrary.Vector_Distance` _array_element (`self.K2_GetActorLocation` _array_element_2)))))
    (if (< (`local.DistantBee`) (`local.NearestBee`))
      (set `local.MinIdx` _array_index)
      (set `local.DistantBee` (`local.NearestBee`))))
  (return (`local.MinIdx`)))

(fn `SpawnBee`
  (params (SpawnTransform :type "Transform Structure") (IsActorSpawn :type Boolean))
  (bind _returnvalue (`|SpawnActorFromClass` "/Game/BeeKeeper/Gentic/Blueprints/BP_BeeProp.BP_BeeProp_C" SpawnTransform "Undefined" "OverrideRootScale" null (`local.IsActorSpawn`) null))
  (bind _returnvalue_2 (`self.CreateBeeGenetic`))
  (`/Game/BeeKeeper/Gentic/Blueprints/BP_BeeProp.UpdateBeeProps` _returnvalue _returnvalue_2 "BeeProp_Restored")
  (add `self.OnDestroyed` _returnvalue (`|CreateDelegate` :!event `BeeDestroyed`))
  (`KismetArrayLibrary.Array_Add` (`self.SpawnedBees`) _returnvalue)
  (`/Game/BeeKeeper/Gentic/Blueprints/BP_BeeProp.InitSim` _returnvalue (`self.K2_GetActorLocation`)))

(fn `UserConstructionScript`)