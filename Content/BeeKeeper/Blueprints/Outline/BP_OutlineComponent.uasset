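; BP_OutlineComponent toggles an outline highlight on a mesh by setting or clearing the M_Outline overlay material.
; When enabling, an optional OutlineSelector maps the hit component to the mesh to highlight; both are supplied through InitComponent.
; It caches the last hit component to report repeated hits, with a manual-update flag that makes the next repeat check return false once.
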(fn `EnableOutline`
  (params (Enable :type Boolean) (HitComponent :type "PrimitiveComponent Object Reference"))
  (bind _outlineselector (`self.OutlineSelector`))
  (if Enable
    (`/Engine/EditorBlueprintResources/StandardMacros.IsValid` (`KismetSystemLibrary.Conv_InterfaceToObject` _outlineselector)
      (:`Is Valid`
        (bind _outlinemesh (`/Game/BeeKeeper/Blueprints/Outline/BPI_OutlineSelector.ComponentHited` _outlineselector HitComponent))
        (bind _output_get (set `self.Mesh` _outlinemesh)))
      (:`Is Not Valid`
        _))
    (`/Engine/EditorBlueprintResources/StandardMacros.IsValid` _output_get
      (:`Is Valid`
        (`MeshComponent.SetOverlayMaterial` (`self.Mesh`) "/Game/BeeKeeper/Materials/Masters/Dummy/M_Outline.M_Outline")))
    (else
      (bind _mesh (`self.Mesh`)
        (:`then`
          (`MeshComponent.SetOverlayMaterial` _mesh null))
        (:`else`)))))

(fn `InitComponent`
  (params (Mesh :type "StaticMeshComponent Object Reference") (OutlineSelector :type "/Game/BeeKeeper/Blueprints/Outline/BPI_OutlineSelector Interface"))
  (set `self.Mesh` Mesh)
  (set `self.OutlineSelector` OutlineSelector))

(fn `IsSelectedComponentHited`
  (params (HitedComponent :type "PrimitiveComponent Object Reference"))
  (returns (Yes :type Boolean))
  (if (== HitedComponent (`self.LastHitComponent`))
    (if (`self.IsManualUpdated`)
      (set `self.IsManualUpdated` false)
      (return false)
      (else
        (return true)))
    (else
      (set `self.LastHitComponent` (`local.HitedComponent`))
      (return false))))

(fn `ManualUpdateIfSelectedLastHit`
  (params (SelectedObj :type "Object Object Reference"))
  (if (== SelectedObj (`self.LastHitComponent`))
    (set `self.IsManualUpdated` true)))