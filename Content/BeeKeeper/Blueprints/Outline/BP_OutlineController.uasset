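; BP_OutlineController is a component that highlights the outlineable object in front of an assigned trace source.
; Each tick it runs a short Visibility line trace along the source's forward vector and moves the highlight to the hit actor's BP_OutlineComponent.
; The highlight clears when the trace hits nothing, but persists when it hits an actor without that component.
; Functions toggle ticking and report whether anything is selected.
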(event `self.ReceiveTick`
  (params (DeltaSeconds :type "Float (single-precision)"))
  (`self.TryOutline`))

(fn `EnableOutlineProc`
  (params (Enable :type Boolean))
  (`self.SetComponentTickEnabled` Enable))

(fn `IsInteractableObjectSelected`
  (returns (Yes :type Boolean))
  (return (`KismetSystemLibrary.IsValid` (`self.CurOutline`))))

(fn `SetTraceSource`
  (params (Source :type "SceneComponent Object Reference"))
  (set `self.TraceSource` Source))

(fn `SwitchOutlineMode`
  (params (bEnabled :type Boolean))
  (if (not bEnabled)
    (bind _curoutline (`self.CurOutline`)
      (:`then`
        (`/Game/BeeKeeper/Blueprints/Outline/BP_OutlineComponent.EnableOutline` _curoutline false)
        (set `self.CurOutline` null))
      (:`else`
        _)))
  (`self.SetComponentTickEnabled` bEnabled))

(fn `TryOutline`
  (bind _tracesource (`self.TraceSource`))
  (bind _returnvalue (`SceneComponent.K2_GetComponentLocation` _tracesource))
  (bind (_outhit _returnvalue_2) (`KismetSystemLibrary.LineTraceSingle` _returnvalue (+ _returnvalue (* (`SceneComponent.GetForwardVector` _tracesource) 150.0)) "TraceTypeQuery1"))
  (if _returnvalue_2
    (bind _returnvalue_3 (`Actor.GetComponentByClass` (`.HitActor` (`GameplayStatics.BreakHitResult` _outhit)) "/Game/BeeKeeper/Blueprints/Outline/BP_OutlineComponent.BP_OutlineComponent_C"))
    (if (and (`KismetSystemLibrary.IsValid` _returnvalue_3) (!= _returnvalue_3 (`self.CurOutline`)))
      (bind _curoutline (`self.CurOutline`)
        (:`then`
          (`/Game/BeeKeeper/Blueprints/Outline/BP_OutlineComponent.EnableOutline` _curoutline false))
        (:`else`
          _))
      (bind _output_get (set `self.CurOutline` _returnvalue_3))
      (`/Game/BeeKeeper/Blueprints/Outline/BP_OutlineComponent.EnableOutline` _output_get true))
    (else
      (bind _curoutline_2 (`self.CurOutline`)
        (:`then`
          (`/Game/BeeKeeper/Blueprints/Outline/BP_OutlineComponent.EnableOutline` _curoutline_2 false)
          (set `self.CurOutline` null))
        (:`else`)))))