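; Beehive frame actor that can be outlined, interacted with, and animated as it is inserted into or removed from its parent actor.
; Timelines slide it vertically, then toward the player camera on removal, toggling an Interact.Moving tag, updating the parent's prompt and firing inserted/removed callbacks.
; Honeycomb texture is set via dynamic material; progress sums FrameData honeycomb values over 100.
; InitFrame is empty, leaving its random species-fill logic disconnected.
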(event `self.ReceiveBeginPlay`
  (`/Game/BeeKeeper/Blueprints/Outline/BP_OutlineComponent.InitComponent` (`self.BP_OutlineComponent`) (`self.Frame`) null)
  (`self.InitFrame`))

(event `StartMoveFrame`
  (params (Z :type "Float (double-precision)" :default -70.0) (NewRate :type "Float (single-precision)" :default 1.0))
  (bind _returnvalue (`self.K2_GetActorLocation`))
  (`BlueprintGameplayTagLibrary.AddGameplayTag` (`self.TagsContainer`) (struct :`TagName` "Interact.Moving"))
  (`TimelineComponent.SetPlayRate` (`self.MoveFrame`) NewRate)
  (message `/Game/BeeKeeper/Blueprints/Interactable/BPI_Interactable.UpdateInteractState` (`self.GetAttachParentActor`))
  (set `self.MoveFromPos` _returnvalue)
  (set `self.MoveToPos` (+ _returnvalue (`KismetMathLibrary.MakeVector` 0.0 0.0 Z)))
  (bind (_direction _zpos) (`Timeline|MoveFrame`)
    (:`Update`
      (`self.K2_SetActorLocation` (`KismetMathLibrary.VLerp` (`self.MoveFromPos`) (`self.MoveToPos`) _zpos)))
    (:`Finished`
      (bind _returnvalue_2 (`BlueprintGameplayTagLibrary.RemoveGameplayTag` (`self.TagsContainer`) (struct :`TagName` "Interact.Moving")))
      (message `/Game/BeeKeeper/Blueprints/Interactable/BPI_Interactable.UpdateInteractState` (`self.GetAttachParentActor`))
      (`self.FrameInserted`)
      (if (not _returnvalue_2)
        (`KismetSystemLibrary.PrintString` "Tag moving removed before")))))

(event `StartRemoveFrame`
  (bind _returnvalue (`self.K2_GetActorLocation`))
  (`BlueprintGameplayTagLibrary.AddGameplayTag` (`self.TagsContainer`) (struct :`TagName` "Interact.Moving"))
  (message `/Game/BeeKeeper/Blueprints/Interactable/BPI_Interactable.UpdateInteractState` (`self.GetAttachParentActor`))
  (set `self.MoveFromPos` _returnvalue)
  (set `self.MoveToPos` (+ _returnvalue (0.0 0.0 70.0)))
  (bind (_direction _zpos) (`Timeline|RemoveFrame` :!via `ReverseFromEnd`)
    (:`Update`
      (`self.K2_SetActorLocation` (`KismetMathLibrary.VLerp` (`self.MoveToPos`) (`self.MoveFromPos`) _zpos)))
    (:`Finished`
      (bind (_direction_2 _zpos_2) (`Timeline|RemoveFrameScale`)
        (:`Update`
          (`self.K2_SetActorLocation` (`KismetMathLibrary.VLerp` (`self.K2_GetActorLocation` (`GameplayStatics.GetPlayerCameraManager` 0)) (`self.MoveToPos`) _zpos_2)))
        (:`Finished`
          (bind _returnvalue_2 (`BlueprintGameplayTagLibrary.RemoveGameplayTag` (`self.TagsContainer`) (struct :`TagName` "Interact.Moving")))
          (if (not _returnvalue_2)
            (`KismetSystemLibrary.PrintString` "Tag moving removed before"))
          (`self.FrameRemoved` self))))))

(event `SetFrameTexture`
  (params (Texture :type "Texture Object Reference"))
  (bind _returnvalue (`PrimitiveComponent.CreateDynamicMaterialInstance` (`self.Frame`) 1 "/Game/BeeKeeper/Materials/Masters/Honeycomb/M_Honeycomb.M_Honeycomb" "None"))
  (`MaterialInstanceDynamic.SetTextureParameterValue` _returnvalue "CombTexture" Texture))

(event `/Game/BeeKeeper/Blueprints/Interactable/BPI_Interactable.Interact`
  (`self.FrameRemoved` self)
  (`self.K2_DestroyActor`))

(fn `GetFrameProgress`
  (returns (Value :type "Float (double-precision)"))
  (locals (Sum :type Integer))
  (bind _values (`BlueprintMapLibrary.Map_Values` (`.Honeycombs_11_CF7265A945E098E2D0E51F8BAF63BA69` (break `/Game/BeeKeeper/Blueprints/Inventory/S_FrameData` (`self.FrameData`)))))
  (for _array_element _values
    (set `local.Sum` (+ _array_element (`local.Sum`))))
  (return (/ (`local.Sum`) 100)))

(fn `InitFrame`
  (locals (AllSpecies :type "Array of Species Enum")))

(fn `Inspect`
  (returns (Yes :type Boolean))
  (return false))

(fn `IsInspectable`
  (returns (Yes :type Boolean))
  (return false))

(fn `UserConstructionScript`)