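; BP_ExtractorDNA is an interactable building that consumes bees from its inventory to extract DNA points, which are currently only printed.
; A looping timer advances progress on the bee in the last slot, removes it when done, then shifts queued bees forward.
; Bound update events drive the player's slot UI, progress bar and a Niagara effect with that bee's material.
; Bees, slots and progress persist through the game instance's save data.
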(event `SetParticleMaterial`
  (bind _bp_inventory (`self.BP_Inventory`))
  (bind _slots (`/Game/BeeKeeper/Inventory/Blueprints/BP_Inventory.Slots` _bp_inventory))
  (bind _asbp_bee_game_instance (cast `/Game/BeeKeeper/Blueprints/BP_BeeGameInstance` (`GameplayStatics.GetGameInstance`) :!label _label))
  (bind _dmi (`/Game/BeeKeeper/Blueprints/BP_BeeGameInstance.GetDMIBeeParticle` _asbp_bee_game_instance (`BeeGenetic.Main` (`|GetArrayItem` (`/Game/BeeKeeper/Inventory/Blueprints/BP_Inventory.Bees` _bp_inventory) (`.InventoryIdx_5_579F21AC4D8636E5B62930970C700287` (break `/Game/BeeKeeper/Blueprints/Inventory/S_SlotData` (`|GetArrayItem` _slots (`KismetArrayLibrary.Array_LastIndex` _slots))))))))
  (`NiagaraComponent.SetVariableMaterial` (`self.NS_MoveInSphere`) "BeeMat" _dmi))

(event `ActivateParticle`
  (bind _ns_moveinsphere (`self.NS_MoveInSphere`))
  (if (not (`ActorComponent.IsActive` _ns_moveinsphere))
    (`ActorComponent.Activate` _ns_moveinsphere false)
    (goto _label)))

(event `self.ReceiveBeginPlay`
  (`/Game/BeeKeeper/Inventory/Blueprints/BP_Inventory.InitSlots` (`self.BP_Inventory`) 9 "NewEnumerator1" false)
  (`/Game/BeeKeeper/Blueprints/Outline/BP_OutlineComponent.InitComponent` (`self.BP_OutlineComponent`) (`self.Cube`) null)
  (add `/Game/BeeKeeper/Inventory/Blueprints/BP_Inventory.SlotChanged` (`self.BP_Inventory`) (`|CreateDelegate` :!event `UpdateInventorySlots`))
  (`KismetSystemLibrary.K2_SetTimerDelegate` (delegate `TickBee`) (`self.ExctractorDnaDelta`) true)
  (add `self.UpdateProgress` (delegate `ActivateParticle`)))

(event `TickBee`
  (bind _bp_inventory (`self.BP_Inventory`))
  (bind _ns_moveinsphere (`self.NS_MoveInSphere`))
  (bind _bp_inventory_2 (`self.BP_Inventory`))
  (bind _slots (`/Game/BeeKeeper/Inventory/Blueprints/BP_Inventory.Slots` _bp_inventory))
  (bind _bees (`/Game/BeeKeeper/Inventory/Blueprints/BP_Inventory.Bees` _bp_inventory))
  (bind _slots_2 (`/Game/BeeKeeper/Inventory/Blueprints/BP_Inventory.Slots` (`self.BP_Inventory`)))
  (bind _slots_3 (`/Game/BeeKeeper/Inventory/Blueprints/BP_Inventory.Slots` (`self.BP_Inventory`)))
  (bind _returnvalue (`KismetArrayLibrary.Array_LastIndex` _slots))
  (bind _output (`|GetArrayItem` _slots _returnvalue))
  (bind (_type _inventoryidx) (break `/Game/BeeKeeper/Blueprints/Inventory/S_SlotData` _output))
  (if (`/Game/BeeKeeper/Blueprints/BPF_Utils.Has Slot Item` (`|GetArrayItem` _slots_3 (`KismetArrayLibrary.Array_LastIndex` _slots_3)))
    (set `self.BeeProgress` (+ (`self.BeeProgress`) (`self.ExctractorDnaDelta`)))
    (`self.UpdateProgress`)
    (if (> (`self.BeeProgress`) (`self.BeeReleaseTime`))
      (set `self.BeeProgress` 0.0)
      (bind _returnvalue_2 (`InheritMutationLibrary.GetDNAPoints` (`|GetArrayItem` _bees _inventoryidx)))
      (`KismetSystemLibrary.PrintText` (`|FormatText` "Add {0} DNA points" _returnvalue_2))
      (`KismetArrayLibrary.Array_Remove` _bees _inventoryidx)
      (`/Game/BeeKeeper/Inventory/Blueprints/BP_Inventory.UpdateSlotsIdxAfterRemove` _bp_inventory_2 (`/Game/BeeKeeper/Inventory/Blueprints/BP_Inventory.Slots` _bp_inventory_2) "NewEnumerator1" _inventoryidx)
      (setmembers `/Game/BeeKeeper/Blueprints/Inventory/S_SlotData` :`StructRef` _output :`InventoryIdx` -1)
      (`self.UpdateInventorySlots` _returnvalue)
      (if (`/Game/BeeKeeper/Blueprints/BPF_Utils.Has Slot Item` (`|GetArrayItem` _slots_2 (`KismetArrayLibrary.Array_LastIndex` _slots_2)))
        (`self.SetParticleMaterial`)))
    (else
      (set `self.BeeProgress` 0.0)
      (if (`ActorComponent.IsActive` _ns_moveinsphere)
        (`ActorComponent.Deactivate` _ns_moveinsphere)))))

(event `/Game/BeeKeeper/Blueprints/PlayerBase/BPI_Buildings.DestroyingBuilding`
  ;[1 1 1] TODO
)

(event `/Game/BeeKeeper/Blueprints/PlayerBase/BPI_Buildings.SaveBuildingData`
  (bind _asbp_bee_game_instance (cast `/Game/BeeKeeper/Blueprints/BP_BeeGameInstance` (`GameplayStatics.GetGameInstance`)))
  (bind _beesdata (`/Game/BeeKeeper/Blueprints/BPF_Utils.GetBeesDataFromBees` (`/Game/BeeKeeper/Inventory/Blueprints/BP_Inventory.Bees` (`self.BP_Inventory`))))
  (`KismetArrayLibrary.Array_Add` (`/Game/BeeKeeper/Blueprints/SaveGame/BP_SaveGame.ExtractorDNASave` (`/Game/BeeKeeper/Blueprints/BP_BeeGameInstance.SaveData` _asbp_bee_game_instance)) (make `/Game/BeeKeeper/Blueprints/SaveGame/S_ExtractorDNASave` _beesdata (`/Game/BeeKeeper/Inventory/Blueprints/BP_Inventory.Slots` (`self.BP_Inventory`)) (`self.GetTransform`) (`self.BeeProgress`))))

(event `/Game/BeeKeeper/Blueprints/Interactable/BPI_Interactable.Interact`
  (bind _asbp_first_person_controller (cast `/Game/BeeKeeper/Blueprints/FirstPersonController/BP_FirstPersonController` (`GameplayStatics.GetPlayerCharacter` 0)))
  (`/Game/BeeKeeper/Blueprints/FirstPersonController/BP_FirstPersonController.ToggleInveontory` _asbp_first_person_controller "NewEnumerator0"))

(event `UpdateProgressBar`
  (bind _asbp_first_person_controller (cast `/Game/BeeKeeper/Blueprints/FirstPersonController/BP_FirstPersonController` (`GameplayStatics.GetPlayerCharacter` 0)))
  (bind _slots (`/Game/BeeKeeper/UI/WB_BeeHiveSelect.Slots` (`/Game/BeeKeeper/UI/WB_HandInventory.WB_BeeHiveSelect` (`/Game/BeeKeeper/Blueprints/FirstPersonController/BP_FirstPersonController.WB_HandInventoryRef` _asbp_first_person_controller))))
  (`ProgressBar.SetPercent` (`/Game/BeeKeeper/UI/WB_HexSlot.ProgressBar` (`|GetArrayItem` _slots (`KismetArrayLibrary.Array_LastIndex` _slots))) (/ (`self.BeeProgress`) (`self.BeeReleaseTime`))))

(event `/Game/BeeKeeper/Blueprints/Interactable/BPI_Interactable.SwitchUiAfterIneract`
  (params (IsUiModeActive :type Boolean))
  (if IsUiModeActive
    (bind _asbp_first_person_controller (cast `/Game/BeeKeeper/Blueprints/FirstPersonController/BP_FirstPersonController` (`GameplayStatics.GetPlayerCharacter` 0)))
    (bind _wb_handinventoryref (`/Game/BeeKeeper/Blueprints/FirstPersonController/BP_FirstPersonController.WB_HandInventoryRef` _asbp_first_person_controller))
    (bind _wb_inventory (`/Game/BeeKeeper/UI/WB_HandInventory.WB_Inventory` _wb_handinventoryref))
    (`/Game/BeeKeeper/UI/WB_Inventory.DisplayBees` _wb_inventory)
    (`/Game/BeeKeeper/UI/WB_Inventory.SwitchSelectTypes` _wb_inventory false)
    (`/Game/BeeKeeper/UI/WB_BeeHiveSelect.DisplayExtractorDnaSlots` (`/Game/BeeKeeper/UI/WB_HandInventory.WB_BeeHiveSelect` _wb_handinventoryref))
    (add `self.UpdateUI` (delegate `UpdatePlayerUI`))
    (add `self.UpdateProgress` (delegate `UpdateProgressBar`))
    (else
      (remove `self.UpdateUI` (delegate `UpdatePlayerUI`))
      (remove `self.UpdateProgress` (delegate `UpdateProgressBar`)))))

(event `UpdatePlayerUI` :!signature `self.UpdateUI`
  (params (Idx :type Integer) (ChangedIdx :type Integer))
  (bind _asbp_first_person_controller (cast `/Game/BeeKeeper/Blueprints/FirstPersonController/BP_FirstPersonController` (`GameplayStatics.GetPlayerCharacter` 0)))
  (bind _wb_beehiveselect (`/Game/BeeKeeper/UI/WB_HandInventory.WB_BeeHiveSelect` (`/Game/BeeKeeper/Blueprints/FirstPersonController/BP_FirstPersonController.WB_HandInventoryRef` _asbp_first_person_controller)))
  (`/Game/BeeKeeper/UI/WB_BeeHiveSelect.DisplayExtractorDnaSlots` _wb_beehiveselect)
  (if (!= Idx -1)
    (`/Game/BeeKeeper/UI/WB_BeeHiveSelect.SetSelectedFrameIcon` _wb_beehiveselect Idx)
    (elif (not (`Widget.IsVisible` (`/Game/BeeKeeper/UI/WB_BeeHiveSelect.SlotFrameIcon` _wb_beehiveselect)))
      (bind _idx (`/Game/BeeKeeper/UI/WB_BeeHiveSelect.GetSelectedIdx` _wb_beehiveselect true))
      (if (and (== _idx ChangedIdx) (`/Game/BeeKeeper/Blueprints/BPF_Utils.Has Slot Item` (`|GetArrayItem` (`/Game/BeeKeeper/Inventory/Blueprints/BP_Inventory.Slots` (`self.BP_Inventory`)) ChangedIdx)))
        (`/Game/BeeKeeper/UI/WB_BeeHiveSelect.EnableFocusSelection` _wb_beehiveselect true)
        (`/Game/BeeKeeper/UI/WB_BeeHiveSelect.SetSelectedFrameIcon` _wb_beehiveselect ChangedIdx)))))

(fn `GetFirstSlotEmptyIdx`
  (returns (Idx :type Integer))
  (bind _slots (`/Game/BeeKeeper/Inventory/Blueprints/BP_Inventory.Slots` (`self.BP_Inventory`)))
  (bind _returnvalue (`KismetArrayLibrary.Array_LastIndex` _slots))
  (if (`/Game/BeeKeeper/Blueprints/BPF_Utils.Has Slot Item` (`|GetArrayItem` _slots _returnvalue))
    (for (_array_element _array_index) (`/Game/BeeKeeper/Inventory/Blueprints/BP_Inventory.Slots` (`self.BP_Inventory`))
      (if (not (`/Game/BeeKeeper/Blueprints/BPF_Utils.Has Slot Item` _array_element))
        (return _array_index)))
    (return -1)
    (else
      (return _returnvalue))))

(fn `Inspect`
  (returns (Yes :type Boolean))
  (return false))

(fn `IsBuilding`
  (returns (Building :type Boolean))
  (return true))

(fn `LoadFromSaveFile`
  (params (Save :type "/Game/BeeKeeper/Blueprints/SaveGame/S_ExtractorDNASave Structure"))
  (bind (_bees _slots _transform _beeprogress) (break `/Game/BeeKeeper/Blueprints/SaveGame/S_ExtractorDNASave` Save))
  (bind _slots_2 (`/Game/BeeKeeper/Inventory/Blueprints/BP_Inventory.Slots` (`self.BP_Inventory`)))
  (`|ExecutionSequence`
    (:`then_0`
      ;[1 1 1] TODO: move this to utlis
      (for _array_element _bees
        (bind _returnvalue (`BeeGenetic.Construct` (break `/Game/BeeKeeper/Blueprints/SaveGame/S_BeeSaveData` _array_element) (`.Sec_5_C70A1CC548EDFF1A1775FE9F61A6EAE7` (break `/Game/BeeKeeper/Blueprints/SaveGame/S_BeeSaveData` _array_element)) (`.Speed_8_1CD6901A441796C254201C907A2497F4` (break `/Game/BeeKeeper/Blueprints/SaveGame/S_BeeSaveData` _array_element)) (`.Fertility_10_F818F0FA45FF2E27C128FE84F2FF8922` (break `/Game/BeeKeeper/Blueprints/SaveGame/S_BeeSaveData` _array_element))))
        (`KismetArrayLibrary.Array_Add` (`/Game/BeeKeeper/Inventory/Blueprints/BP_Inventory.Bees` (`self.BP_Inventory`)) _returnvalue)))
    (:`then_1`
      (set `/Game/BeeKeeper/Inventory/Blueprints/BP_Inventory.Slots` _slots (`self.BP_Inventory`))
      (set `self.BeeProgress` _beeprogress))
    (:`then_2`
      (if (`/Game/BeeKeeper/Blueprints/BPF_Utils.Has Slot Item` (`|GetArrayItem` _slots_2 (`KismetArrayLibrary.Array_LastIndex` _slots_2)))
        (`self.SetParticleMaterial`)))))

(fn `UpdateInventorySlots`
  (params (Idx :type Integer))
  (locals (FirstEmptySlotIdx :type Integer) (SelIdx :type Integer :default -1))
  (bind _slots (`/Game/BeeKeeper/Inventory/Blueprints/BP_Inventory.Slots` (`self.BP_Inventory`)))
  (bind _idx (`self.GetFirstSlotEmptyIdx`))
  (bind _output_get (set `local.FirstEmptySlotIdx` _idx))
  (if (!= _output_get -1)
    (`|ExecutionSequence`
      (:`then_0`
        (for _index (range (`KismetArrayLibrary.Array_LastIndex` (`/Game/BeeKeeper/Inventory/Blueprints/BP_Inventory.Slots` (`self.BP_Inventory`))))
          (bind _output (`|GetArrayItem` (`/Game/BeeKeeper/Inventory/Blueprints/BP_Inventory.Slots` (`self.BP_Inventory`)) _index))
          (if (and (`/Game/BeeKeeper/Blueprints/BPF_Utils.Has Slot Item` _output) (or (> _index (`local.FirstEmptySlotIdx`)) (== (`local.FirstEmptySlotIdx`) (`KismetArrayLibrary.Array_LastIndex` (`/Game/BeeKeeper/Inventory/Blueprints/BP_Inventory.Slots` (`self.BP_Inventory`))))))
            (`KismetArrayLibrary.Array_Set` (`/Game/BeeKeeper/Inventory/Blueprints/BP_Inventory.Slots` (`self.BP_Inventory`)) (`local.FirstEmptySlotIdx`) _output)
            (setmembers `/Game/BeeKeeper/Blueprints/Inventory/S_SlotData` :`StructRef` _output :`InventoryIdx` -1)
            (set `local.SelIdx` (`local.FirstEmptySlotIdx`))
            (if (== (`local.FirstEmptySlotIdx`) (`KismetArrayLibrary.Array_LastIndex` (`/Game/BeeKeeper/Inventory/Blueprints/BP_Inventory.Slots` (`self.BP_Inventory`))))
              (set `local.FirstEmptySlotIdx` 0)
              (elif (!= (`local.FirstEmptySlotIdx`) (- (`KismetArrayLibrary.Array_LastIndex` (`/Game/BeeKeeper/Inventory/Blueprints/BP_Inventory.Slots` (`self.BP_Inventory`))) 1))
                (`/Engine/EditorBlueprintResources/StandardMacros.IncrementInt` (`local.FirstEmptySlotIdx`))
                (else
                  (break)))))))
      (:`then_1`
        (`self.UpdateUI` (`local.SelIdx`) (`local.Idx`)))
      (:`then_2`
        (if (`/Game/BeeKeeper/Blueprints/BPF_Utils.Has Slot Item` (`|GetArrayItem` _slots (`KismetArrayLibrary.Array_LastIndex` _slots)))
          (`self.SetParticleMaterial`))))))

(fn `UserConstructionScript`)