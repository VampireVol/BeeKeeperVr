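; Bee altar building where the player opens the research tree UI by interacting with its table or scroll.
; A request inventory is seeded with honey and wax demands, and submitting research clears stored items, reports completion to the GameInstance and closes the UI.
; ChangeStage swaps wall and table meshes and toggles label, scroll and brick across five stages.
; As outline selector, it highlights the scroll when visible, otherwise the table.
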(event `self.ReceiveBeginPlay`
  (bind _bp_inventory (`self.BP_Inventory`))
  (bind _requestitems (`/Game/BeeKeeper/Inventory/Blueprints/BP_Inventory.RequestItems` _bp_inventory))
  (bind _items (`/Game/BeeKeeper/Inventory/Blueprints/BP_Inventory.Items` _bp_inventory))
  (`/Game/BeeKeeper/Blueprints/Outline/BP_OutlineComponent.InitComponent` (`self.BP_OutlineComponent`) (`self.SM_AltarTable_0`) self)
  (`/Game/BeeKeeper/Inventory/Blueprints/BP_Inventory.InitSlots` (`self.BP_Inventory`) 2 "NewEnumerator0" true)
  (`|ExecutionSequence`
    (:`then_0`
      (`KismetArrayLibrary.Array_Add` _requestitems (make `ItemData` "Honey" 24))
      (`KismetArrayLibrary.Array_Add` _items (make `ItemData` "Honey")))
    (:`then_1`
      (`KismetArrayLibrary.Array_Add` _requestitems (make `ItemData` "Wax" 4))
      (`KismetArrayLibrary.Array_Add` _items (make `ItemData` "Honey")))))

(event `/Game/BeeKeeper/Blueprints/Interactable/BPI_Interactable.Interact`
  (if (or (== (`/Game/BeeKeeper/Blueprints/Outline/BP_OutlineComponent.LastHitComponent` (`self.BP_OutlineComponent`)) (`self.SM_AltarTable_0`)) (== (`/Game/BeeKeeper/Blueprints/Outline/BP_OutlineComponent.LastHitComponent` (`self.BP_OutlineComponent`)) (`self.SM_Scroll`)))
    (bind _asbp_first_person_controller (cast `/Game/BeeKeeper/Blueprints/FirstPersonController/BP_FirstPersonController` (`GameplayStatics.GetPlayerCharacter` 0)))
    (`/Game/BeeKeeper/Blueprints/FirstPersonController/BP_FirstPersonController.ToggleInveontory` _asbp_first_person_controller "NewEnumerator0")))

(event `/Game/BeeKeeper/Blueprints/Interactable/BPI_Interactable.SwitchUiAfterIneract`
  (params (IsUiModeActive :type Boolean))
  (if IsUiModeActive
    (bind _asbp_first_person_controller (cast `/Game/BeeKeeper/Blueprints/FirstPersonController/BP_FirstPersonController` (`GameplayStatics.GetPlayerCharacter` 0)))
    (bind _wb_handinventoryref (`/Game/BeeKeeper/Blueprints/FirstPersonController/BP_FirstPersonController.WB_HandInventoryRef` _asbp_first_person_controller))
    (`Widget.SetVisibility` (`/Game/BeeKeeper/UI/WB_HandInventory.WB_ResearchTree` _wb_handinventoryref) "Visible")
    (bind _wb_beehiveselect (`/Game/BeeKeeper/UI/WB_HandInventory.WB_BeeHiveSelect` _wb_handinventoryref))
    (`Widget.SetVisibility` _wb_beehiveselect "Collapsed")
    (`Widget.SetVisibility` (`/Game/BeeKeeper/UI/WB_HandInventory.WB_Inventory` _wb_handinventoryref) "Collapsed")
    (`Widget.SetVisibility` (`/Game/BeeKeeper/UI/WB_BeeInfoBig.InfoContent` (`/Game/BeeKeeper/UI/WB_HandInventory.WB_BeeInfoBig` _wb_handinventoryref)) "Collapsed")
    (add `/Game/BeeKeeper/UI/WB_BeeHiveSelect.TaskSubmited` _wb_beehiveselect (`|CreateDelegate` :!event `ResearchSubmited`))
    (add `/Game/BeeKeeper/UI/WB_BeeHiveSelect.TaskSubmited` _wb_beehiveselect (`|CreateDelegate` (`/Game/BeeKeeper/UI/WB_HandInventory.WB_ResearchTree` _wb_handinventoryref) :!event `CompleteResearch`))
    (else
      (bind _asbp_first_person_controller_2 (cast `/Game/BeeKeeper/Blueprints/FirstPersonController/BP_FirstPersonController` (`GameplayStatics.GetPlayerCharacter` 0)))
      (bind _wb_handinventoryref_2 (`/Game/BeeKeeper/Blueprints/FirstPersonController/BP_FirstPersonController.WB_HandInventoryRef` _asbp_first_person_controller_2))
      (`Widget.SetVisibility` (`/Game/BeeKeeper/UI/WB_HandInventory.WB_ResearchTree` _wb_handinventoryref_2) "Collapsed")
      (`Widget.SetVisibility` (`/Game/BeeKeeper/UI/WB_HandInventory.WB_Inventory` _wb_handinventoryref_2) "Visible")
      (`Widget.SetVisibility` (`/Game/BeeKeeper/UI/WB_BeeInfoBig.InfoContent` (`/Game/BeeKeeper/UI/WB_HandInventory.WB_BeeInfoBig` _wb_handinventoryref_2)) "Collapsed")
      (bind _wb_beehiveselect_2 (`/Game/BeeKeeper/UI/WB_HandInventory.WB_BeeHiveSelect` _wb_handinventoryref_2))
      (remove `/Game/BeeKeeper/UI/WB_BeeHiveSelect.TaskSubmited` _wb_beehiveselect_2 (`|CreateDelegate` :!event `ResearchSubmited`))
      (remove `/Game/BeeKeeper/UI/WB_BeeHiveSelect.TaskSubmited` _wb_beehiveselect_2 (`|CreateDelegate` (`/Game/BeeKeeper/UI/WB_HandInventory.WB_ResearchTree` _wb_handinventoryref_2) :!event `CompleteResearch`)))))

(fn `ChangeStage`
  (params (Stage :type Integer))
  (bind _returnvalue (== Stage 0))
  (bind _returnvalue_2 (<= Stage 2))
  (bind _sm_goldlable (`self.SM_GoldLable`))
  (bind _sm_brick (`self.SM_Brick`))
  (`|ExecutionSequence`
    (:`then_0`
      (`SceneComponent.SetVisibility` _sm_goldlable _returnvalue false)
      (`SceneComponent.SetVisibility` (`self.SM_Scroll`) (not _returnvalue) false)
      (`PrimitiveComponent.SetCollisionResponseToChannel` _sm_goldlable "ECC_Pawn" (select `bool` _returnvalue :`false` "ECR_Ignore" :`true` "ECR_Block" :!type "ECollisionResponse Enum")))
    (:`then_1`
      (`SceneComponent.SetVisibility` _sm_brick _returnvalue_2 false)
      (`PrimitiveComponent.SetCollisionResponseToChannel` _sm_brick "ECC_Pawn" (select `bool` _returnvalue_2 :`false` "ECR_Ignore" :`true` "ECR_Block" :!type "ECollisionResponse Enum")))
    (:`then_2`
      (`StaticMeshComponent.SetStaticMesh` (`self.SM_Wall_0`) (select `int` Stage :`0` "/Game/BeeKeeper/Meshes/BeeAltar/Stage0/SM_Wall_0.SM_Wall_0" :`1` "/Game/BeeKeeper/Meshes/BeeAltar/Stage1/SM_Wall_1.SM_Wall_1" :`2` "/Game/BeeKeeper/Meshes/BeeAltar/Stage1/SM_Wall_1.SM_Wall_1" :`3` "/Game/BeeKeeper/Meshes/BeeAltar/Stage2/SM_Wall_2.SM_Wall_2" :`4` "/Game/BeeKeeper/Meshes/BeeAltar/Stage3/SM_Wall_3.SM_Wall_3" :!type "StaticMesh Object Reference"))
      (`StaticMeshComponent.SetStaticMesh` (`self.SM_AltarTable_0`) (select `int` Stage :`0` "/Game/BeeKeeper/Meshes/BeeAltar/Stage0/SM_AltarTable_0.SM_AltarTable_0" :`1` "/Game/BeeKeeper/Meshes/BeeAltar/Stage1/SM_AltarTable_1.SM_AltarTable_1" :`2` "/Game/BeeKeeper/Meshes/BeeAltar/Stage2/SM_AltarTable_2.SM_AltarTable_2" :`3` "/Game/BeeKeeper/Meshes/BeeAltar/Stage3/SM_AltarTable_3.SM_AltarTable_3" :`4` "/Game/BeeKeeper/Meshes/BeeAltar/Stage3/SM_AltarTable_3.SM_AltarTable_3" :!type "StaticMesh Object Reference")))))

(fn `ComponentHited`
  (params (HitComponent :type "PrimitiveComponent Object Reference"))
  (returns (OutlineMesh :type "MeshComponent Object Reference"))
  (if (or (== HitComponent (`self.SM_AltarTable_0`)) (== HitComponent (`self.SM_Scroll`)))
    (if (`SceneComponent.IsVisible` (`self.SM_Scroll`))
      (return (`self.SM_Scroll`))
      (else
        (return (`self.SM_AltarTable_0`))))
    (else
      (return null))))

(fn `Inspect`
  (returns (Yes :type Boolean))
  (return false))

(fn `IsBuilding`
  (returns (Building :type Boolean))
  (return true))

(fn `ResearchSubmited`
  (bind _asbp_first_person_controller (cast `/Game/BeeKeeper/Blueprints/FirstPersonController/BP_FirstPersonController` (`GameplayStatics.GetPlayerCharacter` 0)))
  (`|ExecutionSequence`
    (:`then_0`
      (bind _wb_researchtree (`/Game/BeeKeeper/UI/WB_HandInventory.WB_ResearchTree` (`/Game/BeeKeeper/Blueprints/FirstPersonController/BP_FirstPersonController.WB_HandInventoryRef` _asbp_first_person_controller)))
      (message `/Game/BeeKeeper/Blueprints/BPI_GameInstanceTransfer.ResearchComplete` (`GameplayStatics.GetGameInstance`) (`|GetArrayItem` (`/Game/BeeKeeper/UI/WB_ResearchTree.ResearchNames` _wb_researchtree) (`/Game/BeeKeeper/UI/WB_ResearchTree.LastSelectedResearchIdx` _wb_researchtree))))
    (:`then_1`
      (`KismetArrayLibrary.Array_Clear` (`/Game/BeeKeeper/Inventory/Blueprints/BP_Inventory.Items` (`self.BP_Inventory`)))
      (`/Game/BeeKeeper/Blueprints/FirstPersonController/BP_FirstPersonController.DeactivateCurrentUiAndModes` _asbp_first_person_controller "NewEnumerator3"))))

(fn `UserConstructionScript`)