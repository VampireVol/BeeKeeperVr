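; Interactable task board for the beekeeping game that shows tasks in the player's inventory UI and grants rewards for completed ones.
; Interacting toggles the inventory; entering UI mode displays tasks and binds selection and submission events, and leaving restores the previous page and unbinds.
; The last selected task keys a DT_TasksBase lookup, granting an item or a bee with randomized speed and fertility, plus a HUD notification.
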(event `self.ReceiveBeginPlay`
  (`/Game/BeeKeeper/Blueprints/Outline/BP_OutlineComponent.InitComponent` (`self.BP_OutlineComponent`) (`self.Board`) null)
  (`/Game/BeeKeeper/Inventory/Blueprints/BP_Inventory.InitSlots` (`self.BP_Inventory`) 8 "NewEnumerator0" true))

(event `/Game/BeeKeeper/Blueprints/Interactable/BPI_Interactable.Interact`
  (bind _asbp_first_person_controller (cast `/Game/BeeKeeper/Blueprints/FirstPersonController/BP_FirstPersonController` (`GameplayStatics.GetPlayerCharacter` 0)))
  (`/Game/BeeKeeper/Blueprints/FirstPersonController/BP_FirstPersonController.ToggleInveontory` _asbp_first_person_controller "NewEnumerator0"))

(event `/Game/BeeKeeper/Blueprints/Interactable/BPI_Interactable.SwitchUiAfterIneract`
  (params (IsUiModeActive :type Boolean))
  (if IsUiModeActive
    (bind _asbp_first_person_controller (cast `/Game/BeeKeeper/Blueprints/FirstPersonController/BP_FirstPersonController` (`GameplayStatics.GetPlayerCharacter` 0)))
    (bind _wb_handinventoryref (`/Game/BeeKeeper/Blueprints/FirstPersonController/BP_FirstPersonController.WB_HandInventoryRef` _asbp_first_person_controller))
    (bind _wb_inventory (`/Game/BeeKeeper/UI/WB_HandInventory.WB_Inventory` _wb_handinventoryref))
    (`/Game/BeeKeeper/UI/WB_Inventory.DisplayTasks` _wb_inventory)
    (`/Game/BeeKeeper/UI/WB_Inventory.SwitchSelectTypes` _wb_inventory false)
    (bind _wb_beehiveselect (`/Game/BeeKeeper/UI/WB_HandInventory.WB_BeeHiveSelect` _wb_handinventoryref))
    (`Widget.SetVisibility` _wb_beehiveselect "Collapsed")
    (add `/Game/BeeKeeper/UI/WB_Inventory.TaskSelected` _wb_inventory (`|CreateDelegate` :!event `TaskInBoardSelected`))
    (add `/Game/BeeKeeper/UI/WB_BeeHiveSelect.TaskSubmited` _wb_beehiveselect (`|CreateDelegate` :!event `AddRewardForCompletedTask`))
    (else
      (bind _asbp_first_person_controller_2 (cast `/Game/BeeKeeper/Blueprints/FirstPersonController/BP_FirstPersonController` (`GameplayStatics.GetPlayerCharacter` 0)))
      (bind _wb_handinventoryref_2 (`/Game/BeeKeeper/Blueprints/FirstPersonController/BP_FirstPersonController.WB_HandInventoryRef` _asbp_first_person_controller_2))
      (bind _wb_inventory_2 (`/Game/BeeKeeper/UI/WB_HandInventory.WB_Inventory` _wb_handinventoryref_2))
      (set `/Game/BeeKeeper/UI/WB_Inventory.DisplayingType` (`/Game/BeeKeeper/UI/WB_Inventory.LastDisplayingType` _wb_inventory_2) _wb_inventory_2)
      (`/Game/BeeKeeper/UI/WB_Inventory.ValidatePage` _wb_inventory_2)
      (`/Game/BeeKeeper/UI/WB_Inventory.DrawPage` _wb_inventory_2 true)
      (remove `/Game/BeeKeeper/UI/WB_Inventory.TaskSelected` _wb_inventory_2 (`|CreateDelegate` :!event `TaskInBoardSelected`))
      (remove `/Game/BeeKeeper/UI/WB_BeeHiveSelect.TaskSubmited` (`/Game/BeeKeeper/UI/WB_HandInventory.WB_BeeHiveSelect` _wb_handinventoryref_2) (`|CreateDelegate` :!event `AddRewardForCompletedTask`)))))

(event `TaskInBoardSelected`
  (params (TaskName :type Name))
  (set `self.LastSelectedTask` TaskName))

(event `AddRewardForCompletedTask`
  (bind _returnvalue (select `int` (`KismetMathLibrary.RandomInteger` 3) :`0` (`|BitmaskLiteral` 15) :`1` (`|BitmaskLiteral` 60) :`2` (`|BitmaskLiteral` 51)))
  (bind _returnvalue_2 (`|GetDataTableRow` "/Game/BeeKeeper/Blueprints/TasksBoard/DT_TasksBase.DT_TasksBase" (`self.LastSelectedTask`))
    (:`then`
      ;[1 1 1] TODO: make it for VR?
      (bind _asbp_first_person_controller (cast `/Game/BeeKeeper/Blueprints/FirstPersonController/BP_FirstPersonController` (`GameplayStatics.GetPlayerCharacter` 0)))
      (`|ExecutionSequence`
        (:`then_0`
          (bind (_requestitems _rewarditem _rewardbee) (break `TaskData` _returnvalue_2))
          (if (`|EnumInequality` (`.Type` (break `ItemData` _rewarditem)))
            (`/Game/BeeKeeper/Inventory/Blueprints/BP_Inventory.AddItem` (`/Game/BeeKeeper/Blueprints/FirstPersonController/BP_FirstPersonController.BP_Inventory` _asbp_first_person_controller) _rewarditem)
            (bind (_type _count) (break `ItemData` _rewarditem))
            (bind _returnvalue_3 (`/Game/BeeKeeper/Blueprints/BPF_Utils.GetItemIconTexture` _type))
            (bind _wb_playerhud (`/Game/BeeKeeper/Blueprints/FirstPersonController/BP_FirstPersonController.WB PlayerHUD` _asbp_first_person_controller))
            (`/Game/BeeKeeper/UI/WB_PlayerHUD.AddItemNotification` _wb_playerhud _returnvalue_3 (`KismetTextLibrary.Conv_StringToText` (`|GetEnumeratorNameAsString` _type)) _count)
            (else
              (bind _returnvalue_4 (`BeeGenetic.Construct` _rewardbee _rewardbee _returnvalue _returnvalue))
              (`KismetArrayLibrary.Array_Add` (`/Game/BeeKeeper/Inventory/Blueprints/BP_Inventory.Bees` (`/Game/BeeKeeper/Blueprints/FirstPersonController/BP_FirstPersonController.BP_Inventory` _asbp_first_person_controller)) _returnvalue_4)
              (`/Game/BeeKeeper/UI/WB_PlayerHUD.AddBeeNotification` _wb_playerhud _returnvalue_4))))
        (:`then_1`
          (`/Game/BeeKeeper/Blueprints/FirstPersonController/BP_FirstPersonController.ToggleInveontory` _asbp_first_person_controller "NewEnumerator0"))))))

(fn `Inspect`
  (returns (Yes :type Boolean))
  (return false))

(fn `UserConstructionScript`)