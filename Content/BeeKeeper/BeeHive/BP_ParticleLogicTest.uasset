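; BP_ParticleLogicTest is a test actor for the beehive's Niagara bee particle logic.
; On BeginPlay it fills six bee material parameters with per-type dynamic materials from BP_BeeGameInstance, such as River, Forest and Berry.
; It then runs a timed, hardcoded sequence of States changes, converting the enum array to integers and pushing it into the Niagara BeesStates array.
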(event `self.ReceiveBeginPlay`
  (bind _bees (`self.Bees`))
  (bind _asbp_bee_game_instance (cast `/Game/BeeKeeper/Blueprints/BP_BeeGameInstance` (`GameplayStatics.GetGameInstance`)))
  (bind _dmi (`/Game/BeeKeeper/Blueprints/BP_BeeGameInstance.GetDMIBeeParticle` _asbp_bee_game_instance "River"))
  (`NiagaraComponent.SetVariableMaterial` (`self.Bees`) "BeeMat0" _dmi)
  (bind _dmi_2 (`/Game/BeeKeeper/Blueprints/BP_BeeGameInstance.GetDMIBeeParticle` _asbp_bee_game_instance "Forest"))
  (`NiagaraComponent.SetVariableMaterial` (`self.Bees`) "BeeMat1" _dmi_2)
  (bind _dmi_3 (`/Game/BeeKeeper/Blueprints/BP_BeeGameInstance.GetDMIBeeParticle` _asbp_bee_game_instance "Berry"))
  (`NiagaraComponent.SetVariableMaterial` (`self.Bees`) "BeeMat2" _dmi_3)
  (bind _dmi_4 (`/Game/BeeKeeper/Blueprints/BP_BeeGameInstance.GetDMIBeeParticle` _asbp_bee_game_instance "Tomato"))
  (`NiagaraComponent.SetVariableMaterial` (`self.Bees`) "BeeMat3" _dmi_4)
  (bind _dmi_5 (`/Game/BeeKeeper/Blueprints/BP_BeeGameInstance.GetDMIBeeParticle` _asbp_bee_game_instance "Paper"))
  (`NiagaraComponent.SetVariableMaterial` (`self.Bees`) "BeeMat4" _dmi_5)
  (bind _dmi_6 (`/Game/BeeKeeper/Blueprints/BP_BeeGameInstance.GetDMIBeeParticle` _asbp_bee_game_instance "Meadow"))
  (`NiagaraComponent.SetVariableMaterial` (`self.Bees`) "BeeMat5" _dmi_6)
  (`KismetSystemLibrary.Delay` 5.0)
  (bind _statesraw1 (`self.ConvertStatesToIntArray`))
  (`NiagaraDataInterfaceArrayFunctionLibrary.SetNiagaraArrayInt32` _bees "BeesStates" _statesraw1)
  (`KismetSystemLibrary.Delay` 5.0)
  (set `self.States` (`|MakeArray` "NewEnumerator2" "NewEnumerator1" "NewEnumerator2" "NewEnumerator1" "NewEnumerator0" "NewEnumerator1" :!type "/Game/BeeKeeper/FX/E_BeesParticleState Enum"))
  (bind _statesraw1_2 (`self.ConvertStatesToIntArray`))
  (`NiagaraDataInterfaceArrayFunctionLibrary.SetNiagaraArrayInt32` _bees "BeesStates" _statesraw1_2)
  (`KismetSystemLibrary.Delay` 2.0)
  (set `self.States` (`|MakeArray` "NewEnumerator2" "NewEnumerator0" "NewEnumerator2" "NewEnumerator0" "NewEnumerator0" "NewEnumerator0" :!type "/Game/BeeKeeper/FX/E_BeesParticleState Enum"))
  (bind _statesraw1_3 (`self.ConvertStatesToIntArray`))
  (`NiagaraDataInterfaceArrayFunctionLibrary.SetNiagaraArrayInt32` _bees "BeesStates" _statesraw1_3))

(fn `ConvertStatesToIntArray`
  (returns (StatesRaw1 :type "Array of Integer"))
  (locals (StatesRaw :type "Array of Integer"))
  (for _array_element (`self.States`)
    (`KismetArrayLibrary.Array_Add` (`local.StatesRaw`) (`KismetMathLibrary.Conv_ByteToInt` _array_element)))
  (return (`local.StatesRaw`)))

(fn `UserConstructionScript`)