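; VR beehive actor that breeds two bee props placed in its left and right spheres, first as queen, second as drone.
; Overlaps ignore inventory-held bees, copy genetics and tint the spheres; once paired, hearts play during a short timer before both props are destroyed.
; A repeating timer then breeds inherited offspring up to the queen's fertility, updating a camera-facing stats widget with progress, icons and productivity.
; ClearBeeHive resets the hive.
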(event `self.ReceiveBeginPlay`
  (bind _aswb_bee_hive_stats (cast `/Game/BeeKeeper/UI/WB_BeeHiveStats` (`WidgetComponent.GetUserWidgetObject` (`self.BeeStats`))))
  (set `/Game/BeeKeeper/UI/WB_BeeHiveStats.BeeHive` self _aswb_bee_hive_stats)
  (set `self.Bee Hive Stats WB` _aswb_bee_hive_stats))

(event `self.BeeSphereRight.OnComponentBeginOverlap`
  (params (OverlappedComponent :type "PrimitiveComponent Object Reference") (OtherActor :type "Actor Object Reference") (OtherComp :type "PrimitiveComponent Object Reference") (OtherBodyIndex :type Integer) (bFromSweep :type Boolean) (SweepResult :type "HitResult Structure (by ref)"))
  (bind _returnvalue (`KismetSystemLibrary.GetObjectName` OtherActor))
  (bind _asbp_bee_prop (cast `/Game/BeeKeeper/Gentic/Blueprints/BP_BeeProp` OtherActor))
  (bind _valid (`self.CheckInventorySpheresBeeProp` _returnvalue))
  (if (and _valid (`KismetStringLibrary.IsEmpty` (`self.RightSphereActor`)) (`KismetSystemLibrary.IsValid` (`self.GetComponentByClass` OtherActor "/Script/BeeKeeperVr.BeeGenetic")) (`KismetStringLibrary.NotEqual_StrStr` _returnvalue (`self.LeftSphereActor`)))
    (set `self.RightSphereActor` _returnvalue)
    (set `self.IsRightQueen` (not (`self.QueenBeeSelected`)))
    (`self.CheckBeginOverlap` (`self.RightSphereMaterial`) (`/Game/BeeKeeper/Gentic/Blueprints/BP_BeeProp.BeeGenetic` _asbp_bee_prop))))

(event `self.BeeSphereLeft.OnComponentBeginOverlap`
  (params (OverlappedComponent :type "PrimitiveComponent Object Reference") (OtherActor :type "Actor Object Reference") (OtherComp :type "PrimitiveComponent Object Reference") (OtherBodyIndex :type Integer) (bFromSweep :type Boolean) (SweepResult :type "HitResult Structure (by ref)"))
  (bind _returnvalue (`KismetSystemLibrary.GetObjectName` OtherActor))
  (bind _asbp_bee_prop (cast `/Game/BeeKeeper/Gentic/Blueprints/BP_BeeProp` OtherActor))
  (bind _valid (`self.CheckInventorySpheresBeeProp` _returnvalue))
  (if (and _valid (`KismetStringLibrary.IsEmpty` (`self.LeftSphereActor`)) (`KismetStringLibrary.NotEqual_StrStr` _returnvalue (`self.RightSphereActor`)) (`KismetSystemLibrary.IsValid` (`self.GetComponentByClass` OtherActor "/Script/BeeKeeperVr.BeeGenetic")))
    (set `self.LeftSphereActor` _returnvalue)
    (set `self.IsRightQueen` (`self.QueenBeeSelected`))
    (`self.CheckBeginOverlap` (`self.LeftSphereMaterial`) (`/Game/BeeKeeper/Gentic/Blueprints/BP_BeeProp.BeeGenetic` _asbp_bee_prop))))

(event `self.BeeSphereRight.OnComponentEndOverlap`
  (params (OverlappedComponent :type "PrimitiveComponent Object Reference") (OtherActor :type "Actor Object Reference") (OtherComp :type "PrimitiveComponent Object Reference") (OtherBodyIndex :type Integer))
  (if (`KismetStringLibrary.EqualEqual_StrStr` (`KismetSystemLibrary.GetObjectName` OtherActor) (`self.RightSphereActor`))
    (`self.CheckEndOverlap` (`self.RightSphereMaterial`) (`self.LeftSphereMaterial`) (`self.IsRightQueen`))
    (set `self.RightSphereActor` "")))

(event `self.BeeSphereLeft.OnComponentEndOverlap`
  (params (OverlappedComponent :type "PrimitiveComponent Object Reference") (OtherActor :type "Actor Object Reference") (OtherComp :type "PrimitiveComponent Object Reference") (OtherBodyIndex :type Integer))
  (if (`KismetStringLibrary.EqualEqual_StrStr` (`KismetSystemLibrary.GetObjectName` OtherActor) (`self.LeftSphereActor`))
    (`self.CheckEndOverlap` (`self.LeftSphereMaterial`) (`self.RightSphereMaterial`) (not (`self.IsRightQueen`)))
    (set `self.LeftSphereActor` "")))

(event `BeeKissing`
  (bind _returnvalue (`KismetSystemLibrary.K2_SetTimer` null "BeeInherit" 3.0))
  (`ActorComponent.Activate` (`self.ParticalHearts`) true))

(event `BeeNotKissing`
  (`KismetSystemLibrary.K2_ClearAndInvalidateTimerHandle` (stale `BeeKissing` _returnvalue))
  (`ActorComponent.Deactivate` (`self.ParticalHearts`)))

(event `self.ReceiveTick`
  (params (DeltaSeconds :type "Float (single-precision)"))
  (`self.UpdateWidgetRotation`)
  (bind _aswb_bee_hive_stats (cast `/Game/BeeKeeper/UI/WB_BeeHiveStats` (`WidgetComponent.GetUserWidgetObject` (`self.BeeStats`))))
  (set `/Game/BeeKeeper/UI/WB_BeeHiveStats.ProgressPercent` (/ (`KismetSystemLibrary.K2_GetTimerElapsedTimeHandle` (stale `BeeInheritEvent` _returnvalue)) 10.0) _aswb_bee_hive_stats))

(event `BeeInheritEvent`
  (bind _returnvalue (`KismetSystemLibrary.K2_SetTimer` null "BornNewBee" 10.0)))

(event `StopBeeIngeritEvent`
  (`KismetSystemLibrary.K2_ClearAndInvalidateTimerHandle` (stale `BeeInheritEvent` _returnvalue)))

(event `ClearBeeHive`
  (`KismetArrayLibrary.Array_Clear` (`self.Bees`))
  (set `self.CountBeesBorn` 0)
  (set `self.LeftSphereActor` "")
  (set `self.RightSphereActor` "")
  (set `self.SkipOverlap` false)
  (set `self.QueenBeeSelected` false)
  (set `self.DroneBeeSelected` false)
  (set `self.QueenBee` null)
  (set `self.DroneBee` null)
  (`SceneComponent.SetVisibility` (`self.BeeSphereLeft`) true false)
  (`SceneComponent.SetVisibility` (`self.BeeSphereRight`) true false)
  (`SceneComponent.SetVisibility` (`self.BeeStats`) false false)
  (`MaterialInstanceDynamic.SetVectorParameterValue` (`self.RightSphereMaterial`) "SphereColor" (`self.DefaultSphereColor`))
  (`MaterialInstanceDynamic.SetVectorParameterValue` (`self.LeftSphereMaterial`) "SphereColor" (`self.DefaultSphereColor`))
  (bind _aswb_bee_hive_stats (cast `/Game/BeeKeeper/UI/WB_BeeHiveStats` (`WidgetComponent.GetUserWidgetObject` (`self.BeeStats`))))
  (`/Game/BeeKeeper/UI/WB_BeeHiveStats.UpdateProductivityValue` _aswb_bee_hive_stats))

(fn `BeeInherit`
  (bind _beesphereright (`self.BeeSphereRight`))
  (bind _beesphereleft (`self.BeeSphereLeft`))
  (bind _queenbee (`self.QueenBee`))
  (`ActorComponent.Deactivate` (`self.ParticalHearts`))
  (bind _returnvalue (`BeeGenetic.GetInfoBee` _queenbee))
  (bind _returnvalue_2 (`KismetArrayLibrary.Array_Add` (`self.Bees`) _queenbee))
  (bind _widget (`self.GetBeeHiveWidget`))
  (bind _returnvalue_3 (`BeeFunctionLibrary.GetIcon` "/Game/BeeKeeper/BeeModel/DT_Icons.DT_Icons" (`BeeGenetic.Main` _queenbee)))
  (bind _output (`|GetArrayItem` (`/Game/BeeKeeper/UI/WB_BeeHiveStats.BeeIcons` _widget) _returnvalue_2))
  (`Image.SetBrush` _output (`WidgetBlueprintLibrary.MakeBrushFromTexture` _returnvalue_3 128 128))
  (`Widget.SetVisibility` _output "SelfHitTestInvisible")
  (`SceneComponent.SetVisibility` _beesphereright false false)
  (`SceneComponent.SetVisibility` _beesphereleft false false)
  (for _array_element (`PrimitiveComponent.GetOverlappingActors` _beesphereright null)
    (if (`KismetStringLibrary.EqualEqual_StrStr` (`KismetSystemLibrary.GetObjectName` _array_element) (`self.RightSphereActor`))
      (set `self.SkipOverlap` true)
      (`self.K2_DestroyActor` _array_element)
      (break)))
  (for _array_element_2 (`PrimitiveComponent.GetOverlappingActors` _beesphereleft null)
    (if (`KismetStringLibrary.EqualEqual_StrStr` (`KismetSystemLibrary.GetObjectName` _array_element_2) (`self.LeftSphereActor`))
      (`self.K2_DestroyActor` _array_element_2)
      (`SceneComponent.SetVisibility` (`self.BeeStats`) true false)
      (bind _aswb_bee_hive_stats (cast `/Game/BeeKeeper/UI/WB_BeeHiveStats` (`WidgetComponent.GetUserWidgetObject` (`self.BeeStats`))))
      (`/Game/BeeKeeper/UI/WB_BeeHiveStats.SetQueenEvent` _aswb_bee_hive_stats)
      (`self.BeeInheritEvent`)
      (break))))

(fn `BornNewBee`
  (bind _queenbee (`self.QueenBee`))
  (bind _returnvalue (`InheritMutationLibrary.Inherit` _queenbee (`self.DroneBee`)))
  (bind _returnvalue_2 (`KismetArrayLibrary.Array_Add` (`self.Bees`) _returnvalue))
  (bind _widget (`self.GetBeeHiveWidget`))
  (`/Game/BeeKeeper/UI/WB_BeeHiveStats.UpdateProductivityValue` _widget)
  (bind _widget_2 (`self.GetBeeHiveWidget`))
  (bind _returnvalue_3 (`BeeFunctionLibrary.GetIcon` "/Game/BeeKeeper/BeeModel/DT_Icons.DT_Icons" (`BeeGenetic.Main` _returnvalue)))
  (bind _output (`|GetArrayItem` (`/Game/BeeKeeper/UI/WB_BeeHiveStats.BeeIcons` _widget_2) _returnvalue_2))
  (`Image.SetBrush` _output (`WidgetBlueprintLibrary.MakeBrushFromTexture` _returnvalue_3 128 128))
  (`Widget.SetVisibility` _output "SelfHitTestInvisible")
  (bind _output_get (set `self.CountBeesBorn` (+ (`self.CountBeesBorn`) 1)))
  (bind _returnvalue_4 (`BeeGenetic.GetFertiliryValue` _queenbee))
  (if (>= _output_get _returnvalue_4)
    (`self.StopBeeIngeritEvent`)
    (else
      (`self.BeeInheritEvent`))))

(fn `CheckBeginOverlap`
  (params (Material :type "MaterialInstanceDynamic Object Reference") (Bee :type "BeeGenetic Object Reference"))
  (if (`self.SkipOverlap`)
    _
    (elif (`self.QueenBeeSelected`)
      (if (not (`self.DroneBeeSelected`))
        (`MaterialInstanceDynamic.SetVectorParameterValue` Material "SphereColor" (`self.BeeDroneColor`))
        (bind _returnvalue (`InheritMutationLibrary.CopyBeeProps` Bee))
        (set `self.DroneBee` _returnvalue)
        (set `self.DroneBeeSelected` true)
        (`self.BeeKissing`))
      (else
        (`MaterialInstanceDynamic.SetVectorParameterValue` Material "SphereColor" (`self.BeeQueenColor`))
        (bind _returnvalue_2 (`InheritMutationLibrary.CopyBeeProps` Bee))
        (set `self.QueenBee` _returnvalue_2)
        (set `self.QueenBeeSelected` true)))))

(fn `CheckEndOverlap`
  (params (Matreial :type "MaterialInstanceDynamic Object Reference") (AnotherSideMaterial :type "MaterialInstanceDynamic Object Reference") (ThisSphereQueen :type "Boolean (by ref)"))
  (if (`self.SkipOverlap`)
    _
    (elif (and (`self.QueenBeeSelected`) (`self.DroneBeeSelected`))
      (set `self.DroneBeeSelected` false)
      (if ThisSphereQueen
        (if (not (`self.SkipOverlap`))
          (bind _returnvalue (`InheritMutationLibrary.CopyBeeProps` (`self.DroneBee`)))
          (set `self.QueenBee` _returnvalue)
          (`|VariableSetRef` ThisSphereQueen)
          (`MaterialInstanceDynamic.SetVectorParameterValue` AnotherSideMaterial "SphereColor" (`self.BeeQueenColor`))
          (`MaterialInstanceDynamic.SetVectorParameterValue` Matreial "SphereColor" (`self.DefaultSphereColor`) :!label _label)
          (`self.BeeNotKissing`))
        (else
          (goto _label)))
      (else
        (set `self.QueenBeeSelected` false)
        (goto _label)))))

(fn `CheckInventorySpheresBeeProp`
  (params (BeeInputName :type String))
  (returns (Valid :type Boolean))
  (bind (_asvrpawn _bsuccess) (cast `/Game/VRTemplate/Blueprints/VRPawn` (`GameplayStatics.GetPlayerPawn` 0) :!pure true))
  (if _bsuccess
    (return (and (`KismetStringLibrary.NotEqual_StrStr` (`KismetSystemLibrary.GetObjectName` (`ActorComponent.GetOwner` (`/Game/BeeKeeper/Inventory/Blueprints/BP_InventorySlot.ContainedObject` (`/Game/VRTemplate/Blueprints/VRPawn.InventorySlotRightRef` _asvrpawn)))) BeeInputName) (`KismetStringLibrary.NotEqual_StrStr` BeeInputName (`KismetSystemLibrary.GetObjectName` (`ActorComponent.GetOwner` (`/Game/BeeKeeper/Inventory/Blueprints/BP_InventorySlot.ContainedObject` (`/Game/VRTemplate/Blueprints/VRPawn.InventorySlotLeftRef` _asvrpawn)))))))))

(fn `GetBeeHiveWidget`
  (returns (Widget :type "/Game/BeeKeeper/UI/WB_BeeHiveStats Object Reference"))
  (bind _aswb_bee_hive_stats (cast `/Game/BeeKeeper/UI/WB_BeeHiveStats` (`WidgetComponent.GetUserWidgetObject` (`self.BeeStats`))))
  (return _aswb_bee_hive_stats))

(fn `UpdateWidgetRotation`
  (bind _beestats (`self.BeeStats`))
  (bind (_returnvalue_x _returnvalue_y) (`KismetMathLibrary.BreakVector` (- (`SceneComponent.K2_GetComponentLocation` (`/Game/VRTemplate/Blueprints/VRPawn.Camera` (cast `/Game/VRTemplate/Blueprints/VRPawn` (`GameplayStatics.GetPlayerPawn` 0) :!pure true))) (`SceneComponent.K2_GetComponentLocation` _beestats))))
  (if (`SceneComponent.IsVisible` _beestats)
    (`SceneComponent.K2_SetWorldRotation` _beestats (`KismetMathLibrary.MakeRotFromX` (`KismetMathLibrary.Normal` (`KismetMathLibrary.MakeVector` _returnvalue_x _returnvalue_y))) false false)))

(fn `UserConstructionScript`
  (bind _returnvalue (`PrimitiveComponent.CreateDynamicMaterialInstance` (`self.BeeSphereRight`) 0 null "None"))
  (set `self.RightSphereMaterial` _returnvalue)
  (bind _returnvalue_2 (`PrimitiveComponent.CreateDynamicMaterialInstance` (`self.BeeSphereLeft`) 0 null "None"))
  (set `self.LeftSphereMaterial` _returnvalue_2))