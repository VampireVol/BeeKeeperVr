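; Function library of flat-top hex grid math, filed with the BeeKeeper game's beehive assets.
; Converts between axial Q/R coordinates and 2D positions using a hard-coded cell size, and computes hex corner points.
; PixelToHex snaps through cube-coordinate rounding, and GetCenterHex chains both conversions to find a position's cell center.
; RoundHex offers an alternative branchless rounding that no other function here calls.
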(fn `FlatHexCorner`
  (params (CenterX :type "Float (double-precision)") (CenterY :type "Float (double-precision)") (Idx :type Integer))
  (returns (X :type "Float (double-precision)") (Y :type "Float (double-precision)"))
  (bind _returnvalue (* (* Idx 60) (/ (`KismetMathLibrary.GetPI`) 180.0)))
  (bind _gridsize (`self.GetGridSize` null))
  (return (+ CenterX (* (`KismetMathLibrary.Cos` _returnvalue) _gridsize)) (+ CenterY (* (`KismetMathLibrary.Sin` _returnvalue) _gridsize))))

(fn `GetCenterHex`
  (params (X :type "Float (double-precision)") (Y :type "Float (double-precision)"))
  (returns (CenterX :type "Float (double-precision)") (CenterY :type "Float (double-precision)") (NewParam :type Boolean))
  (bind (_q _r) (`self.PixelToHex` X Y))
  (bind (_x _y) (`self.HexToPixel` _q _r))
  (return _x _y false))

(fn `GetGridSize`
  (returns (GridSize :type "Float (double-precision)"))
  (return 50.0))

(fn `HexToPixel`
  (params (Q :type Integer) (R :type Integer))
  (returns (X :type "Float (double-precision)") (Y :type "Float (double-precision)"))
  (bind _returnvalue (`KismetMathLibrary.Sqrt` 3.0))
  (bind _gridsize (`self.GetGridSize` null))
  (return (* _gridsize (* Q 1.5)) (* _gridsize (+ (* Q (/ _returnvalue 2.0)) (* R _returnvalue)))))

(fn `PixelToHex`
  (params (X :type "Float (double-precision)") (Y :type "Float (double-precision)"))
  (returns (Q :type Integer) (R :type Integer))
  (bind _gridsize (`self.GetGridSize` null))
  (bind (_qout _rout) (`self.RoundCubeHex` (/ (* X (/ 2.0 3.0)) _gridsize) (/ (+ (* X (/ -1.0 3.0)) (* Y (/ (`KismetMathLibrary.Sqrt` 3.0) 3.0))) _gridsize)))
  (return _qout _rout))

(fn `RoundCubeHex`
  (params (Q :type "Float (double-precision)") (R :type "Float (double-precision)"))
  (returns (QOut :type Integer) (ROut :type Integer))
  (locals (S :type "Float (double-precision)") (QDiff :type "Float (double-precision)" :default 0.0) (RDiff :type "Float (double-precision)" :default 0.0) (SDiff :type "Float (double-precision)" :default 0.0) (QRound :type Integer :default 0) (RRound :type Integer :default 0) (SRound :type Integer :default 0))
  (bind _output_get (set `local.S` (- 0.0 Q R)))
  (bind _output_get_2 (set `local.QRound` (`KismetMathLibrary.Round` Q)))
  (bind _output_get_3 (set `local.RRound` (`KismetMathLibrary.Round` R)))
  (bind _output_get_4 (set `local.SRound` (`KismetMathLibrary.Round` _output_get)))
  (bind _output_get_5 (set `local.QDiff` (`KismetMathLibrary.Abs` (- Q _output_get_2))))
  (bind _output_get_6 (set `local.RDiff` (`KismetMathLibrary.Abs` (- R _output_get_3))))
  (bind _output_get_7 (set `local.SDiff` (`KismetMathLibrary.Abs` (- (`local.S`) _output_get_4))))
  (if (and (> _output_get_5 _output_get_6) (> _output_get_5 _output_get_7))
    (set `local.QRound` (- 0 (`local.RRound`) (`local.SRound`)))
    (elif (> _output_get_6 _output_get_7)
      (set `local.RRound` (- 0 (`local.QRound`) (`local.SRound`)))
      (else
        (set `local.SRound` (- 0 (`local.QRound`) (`local.RRound`))))))
  (return (`local.QRound`) (`local.RRound`)))

(fn `RoundHex`
  (params (X :type "Float (double-precision)") (Y :type "Float (double-precision)"))
  (returns (Q :type Integer) (R :type Integer))
  (locals (NewLocalVar :type "Float (double-precision)") (XGrid :type Integer :default 0) (YGrid :type Integer :default 0) (`X*X` :type "Float (double-precision)" :default 0.0) (`Y*Y` :type "Float (double-precision)" :default 0.0))
  (bind _returnvalue (`KismetMathLibrary.Round` X))
  (bind _returnvalue_2 (`KismetMathLibrary.Round` Y))
  (bind _returnvalue_3 (- X _returnvalue))
  (bind _returnvalue_4 (- Y _returnvalue_2))
  (set `local.XGrid` _returnvalue)
  (set `local.YGrid` _returnvalue_2)
  (set `local.X*X` (`KismetMathLibrary.Square` _returnvalue_3))
  (set `local.Y*Y` (`KismetMathLibrary.Square` _returnvalue_4))
  (return (+ (`local.XGrid`) (* (`KismetMathLibrary.Round` (+ _returnvalue_4 (* _returnvalue_3 0.5))) (`KismetMathLibrary.Conv_BoolToInt` (>= (`local.X*X`) (`local.Y*Y`))))) (+ (`local.YGrid`) (* (`KismetMathLibrary.Round` (+ _returnvalue_3 (* _returnvalue_4 0.5))) (`KismetMathLibrary.Conv_BoolToInt` (< (`local.X*X`) (`local.Y*Y`)))))))