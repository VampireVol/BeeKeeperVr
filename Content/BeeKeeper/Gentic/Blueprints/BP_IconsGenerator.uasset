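; Offline icon generator actor that renders a PNG icon for every bee species into the hobeey-assets folder.
; On BeginPlay, a SceneCapture2D isolates the bee prop's mesh and hat with show-only components, then captures each species.
; Each capture passes through a material drawn to FinalTarget before export.
; Unconnected chains hold recipes for other item icons and export experiments; GetBeeIcon updates the species and returns a DMI brush without capturing.
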(event `self.ReceiveBeginPlay`
  (bind _scenecapturecomponent2d (`self.SceneCaptureComponent2D`))
  (bind _bp_beeprop (`self.BP_BeeProp`))
  (bind _finaltarget (`self.FinalTarget`))
  ;[1 1 1] Bees Icons
  (`SceneComponent.SetVisibility` _bp_beeprop true false)
  (bind _asbp_bee_prop (cast `/Game/BeeKeeper/Gentic/Blueprints/BP_BeeProp` (`ChildActorComponent.ChildActor` _bp_beeprop)))
  (set `SceneCaptureComponent2D.FOVAngle` 90.0 _scenecapturecomponent2d)
  (for _array_element (`|MakeArray` (`/Game/BeeKeeper/Gentic/Blueprints/BP_BeeProp.StaticMesh` _asbp_bee_prop) (`/Game/BeeKeeper/Gentic/Blueprints/BP_BeeProp.Hat` _asbp_bee_prop))
    (`SceneCaptureComponent.ShowOnlyComponent` _scenecapturecomponent2d _array_element))
  (bind _enumvalue (foreach `Species` false)
    (:`LoopBody`
      (`/Game/BeeKeeper/Gentic/Blueprints/BP_BeeProp.Update Mesh Species` _asbp_bee_prop _enumvalue)
      (`SceneCaptureComponent2D.CaptureScene` (`self.SceneCaptureComponent2D`))
      (`KismetRenderingLibrary.ClearRenderTarget2D` _finaltarget)
      (`KismetRenderingLibrary.DrawMaterialToRenderTarget` _finaltarget (`self.NewVar`))
      (`KismetRenderingLibrary.ExportRenderTarget` _finaltarget (`KismetStringLibrary.Concat_StrStr` (`KismetSystemLibrary.GetProjectDirectory`) "../hobeey-assets/Icons/Generated/Reborn2/") (`KismetStringLibrary.Concat_StrStr` (`|GetEnumeratorNameAsString` _enumvalue) ".png")))))

(event `CustomEvent`
  (params (bSuccess :type Boolean))
  (`KismetSystemLibrary.PrintString` "saved!"))

(event `Complite`
  (params (bSuccess :type Boolean))
  (`KismetSystemLibrary.PrintString` "saved!"))

(fn `GetBeeIcon`
  (params (species :type "Species Enum" :default "Meadow") (`icon size` :type "Vector2D Structure"))
  (returns (ReturnValue :type "SlateBrush Structure"))
  (bind _asbp_bee_prop (cast `/Game/BeeKeeper/Gentic/Blueprints/BP_BeeProp` (`ChildActorComponent.ChildActor` (`self.BP_BeeProp`))))
  (`/Game/BeeKeeper/Gentic/Blueprints/BP_BeeProp.Update Mesh Species` _asbp_bee_prop species)
  (return (`WidgetBlueprintLibrary.MakeBrushFromMaterial` (`self.DMI`) (`KismetMathLibrary.FTrunc` `icon size_X`) (`KismetMathLibrary.FTrunc` `icon size_Y`))))

(fn `UserConstructionScript`)