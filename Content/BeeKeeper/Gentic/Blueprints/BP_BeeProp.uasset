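; Interactable bee actor that shows its genetics, tints its material by species from DT_Icons, and goes into the player's inventory on interact.
; When simulated, Tick steers it between random points around a base point with smoothed velocity and turn assist.
; Inspect pauses flight and uses a timeline to bring it before the camera, where the mouse tilts it; cancelling reverses this.
; It also has a toggleable bobbing crown and date-based winter hat.
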(event `UpdateBeeInfo`
  (bind _asbee_stats_widget (cast `/Game/BeeKeeper/UI/BeeStatsWidget` (`WidgetComponent.GetUserWidgetObject` (`self.InfoWidget`)) :!label _label))
  (`/Game/BeeKeeper/UI/BeeStatsWidget.UpdateInfo` _asbee_stats_widget (`self.BeeGenetic`)))

(event `self.ReceiveBeginPlay`
  (`|ExecutionSequence`
    (:`then_0`
      (if (`self.IsActorSpawn`)
        (`self.SetActorEnableCollision` false))
      (`/Game/BeeKeeper/Blueprints/Outline/BP_OutlineComponent.InitComponent` (`self.BP_OutlineComponent`) (`self.BeeSKM`) null)
      (set `self.CrownPos` (`SceneComponent.RelativeLocation` (`self.Crown`)))
      (goto _label))
    (:`then_1`
      (bind _asabp_bee (cast `/Game/BeeKeeper/Meshes/Bee/ABP_Bee` (`SkeletalMeshComponent.GetAnimInstance` (`self.BeeSKM`))))
      (set `/Game/BeeKeeper/Meshes/Bee/ABP_Bee.StartFlyPos` (`KismetMathLibrary.RandomFloatInRange` 0.0 2.0) _asabp_bee))))

(event `self.ReceiveTick`
  (params (DeltaSeconds :type "Float (single-precision)"))
  (bind (_crownpos_x _crownpos_y _crownpos_z) (`KismetMathLibrary.BreakVector` (`self.CrownPos`)))
  (bind _crown (`self.Crown`))
  (bind (_returnvalue_x _returnvalue_y _returnvalue_z) (`KismetMathLibrary.BreakVector` (`SceneComponent.K2_GetComponentLocation` (`self.BeeSKM`))))
  (bind _returnvalue_location (`KismetMathLibrary.BreakTransform` (`SceneComponent.GetSocketTransform` (`self.BeeSKM`) "BodySocket" "RTS_Actor")))
  (bind (_relativerotation_roll _relativerotation_pitch _relativerotation_yaw) (`KismetMathLibrary.BreakRotator` (`SceneComponent.RelativeRotation` (`self.Crown`))))
  (`self.InspectAct` DeltaSeconds)
  (`self.SimAct` DeltaSeconds)
  (if (`SceneComponent.IsVisible` (`self.Crown`))
    (`SceneComponent.K2_SetRelativeRotation` _crown (`KismetMathLibrary.MakeRotator` _relativerotation_roll _relativerotation_pitch (+ _relativerotation_yaw (* DeltaSeconds 30.0))) false false)
    (`SceneComponent.K2_SetRelativeLocation` _crown (+ (`KismetMathLibrary.MakeVector` _crownpos_x _crownpos_y (+ _crownpos_z (* (`KismetMathLibrary.Sin` (- (* (`GameplayStatics.GetTimeSeconds`) 5.0) (/ (`KismetMathLibrary.GetPI`) 2.0))) 2.0))) _returnvalue_location) false false))
  (if (< _returnvalue_z 0.0)
    (`SceneComponent.K2_SetWorldLocationAndRotation` :`self` (`self.BeeSKM`) :`NewLocation` (`KismetMathLibrary.MakeVector` _returnvalue_x _returnvalue_y 330.0))))

(event `/Game/BeeKeeper/Blueprints/Interactable/BPI_Interactable.Interact`
  (bind _beegenetic (`self.BeeGenetic`))
  (bind _asbp_bee_game_instance (cast `/Game/BeeKeeper/Blueprints/BP_BeeGameInstance` (`GameplayStatics.GetGameInstance`)))
  (`/Game/BeeKeeper/Blueprints/BP_BeeGameInstance.Update Discovered Bees` _asbp_bee_game_instance _beegenetic)
  (bind _returnvalue (`InheritMutationLibrary.CopyBeeProps` _beegenetic))
  (bind _asbp_first_person_controller (cast `/Game/BeeKeeper/Blueprints/FirstPersonController/BP_FirstPersonController` (`GameplayStatics.GetPlayerCharacter` 0)))
  (`KismetArrayLibrary.Array_Add` (`/Game/BeeKeeper/Inventory/Blueprints/BP_Inventory.Bees` (`/Game/BeeKeeper/Blueprints/FirstPersonController/BP_FirstPersonController.BP_Inventory` _asbp_first_person_controller)) _returnvalue)
  (`/Game/BeeKeeper/UI/WB_PlayerHUD.AddBeeNotification` (`/Game/BeeKeeper/Blueprints/FirstPersonController/BP_FirstPersonController.WB PlayerHUD` _asbp_first_person_controller) _returnvalue)
  (`self.K2_DestroyActor`)
  (`/Game/BeeKeeper/UI/WB_Inventory.Select Last Item Of Type` (`/Game/BeeKeeper/UI/WB_HandInventory.WB_Inventory` (`/Game/BeeKeeper/Blueprints/FirstPersonController/BP_FirstPersonController.WB_HandInventoryRef` _asbp_first_person_controller)) "NewEnumerator0"))

(event `BeeTakenInerpolate`
  (bind (_returnvalue_x _returnvalue_y) (`KismetMathLibrary.BreakVector2D` (`WidgetLayoutLibrary.GetViewportSize`)))
  (bind (_direction _alpha) (`Timeline|MoveToInspect` :!via `PlayFromStart` :!label _label_2)
    (:`Update`
      (`self.K2_SetActorLocationAndRotation` (`KismetMathLibrary.VLerp` (`self.StartPos`) (`self.TragetPos`) _alpha) (`KismetMathLibrary.RLerp` (`self.StartRot`) (`self.TargetRot`) _alpha true)))
    (:`Finished`
      (if (`|EnumEquality` _direction "Forward")
        (`PlayerController.SetMouseLocation` (`GameplayStatics.GetPlayerController` 0) (`KismetMathLibrary.FTrunc` (/ _returnvalue_x 2.0)) (`KismetMathLibrary.FTrunc` (/ _returnvalue_y 2.0)))
        (set `self.IsActorInspect` true)
        (else
          (`self.SetBeeTaken` false)
          (set `self.IsActorInspect` false)
          (set `self.IsSimulationActive` (`self.WasSimulationActive`)))))))

(event `/Game/BeeKeeper/Blueprints/Interactable/BPI_Interactable.CancelInspect`
  (goto _label_2 :!via `Reverse`))

(fn `FromColorToLinearColor`
  (params (color :type "Color Structure"))
  (returns (`linear color` :type "LinearColor Structure"))
  (bind (_b _g _r _a) (break `Color` color))
  (return (make `LinearColor` (/ _r 256.0) (/ _g 256.0) (/ _b 256.0) (/ _a 256.0))))

(fn `HideCrown`
  (`SceneComponent.SetVisibility` (`self.Crown`) false false))

(fn `InitSim`
  (params (BasePoint :type "Vector Structure"))
  (set `self.IsSimulationActive` true)
  (set `self.BasePoint` BasePoint)
  (set `self.NextPosPoint` (+ (`self.K2_GetActorLocation`) (* (`self.GetActorForwardVector`) (`KismetMathLibrary.RandomFloatInRange` 30.0 60.0))))
  (set `self.ToPointLenght` (`KismetMathLibrary.VSize` (- (`self.NextPosPoint`) (`self.K2_GetActorLocation`)))))

(fn `Inspect`
  (returns (Yes :type Boolean))
  (`|ExecutionSequence`
    (:`then_0`
      (`self.SetBeeTaken` true)
      (set `self.WasSimulationActive` (`self.IsSimulationActive`))
      (set `self.IsSimulationActive` false)
      (bind _asbp_first_person_controller (cast `/Game/BeeKeeper/Blueprints/FirstPersonController/BP_FirstPersonController` (`GameplayStatics.GetPlayerCharacter` 0)))
      (set `self.StartPos` (`self.K2_GetActorLocation`))
      (set `self.StartRot` (`self.K2_GetActorRotation`))
      (bind _firstpersoncamera (`/Game/BeeKeeper/Blueprints/FirstPersonController/BP_FirstPersonController.FirstPersonCamera` _asbp_first_person_controller))
      (set `self.TragetPos` (+ (`SceneComponent.K2_GetComponentLocation` _firstpersoncamera) (* (`SceneComponent.GetForwardVector` _firstpersoncamera) 35.0)))
      (bind _output_get (set `self.TargetRot` (`KismetMathLibrary.ComposeRotators` (struct :`Pitch` 90.0 :`Yaw` 180.0) (`SceneComponent.K2_GetComponentRotation` _firstpersoncamera))))
      (set `self.TargetBaseRot` _output_get)
      (`self.BeeTakenInerpolate`))
    (:`then_2`
      (return true))))

(fn `InspectAct`
  (params (DeltaTime :type "Float (single-precision)"))
  (bind (_returnvalue_x _returnvalue_y) (`KismetMathLibrary.BreakVector2D` (`WidgetLayoutLibrary.GetViewportSize`)))
  (bind (_locationx _locationy) (`PlayerController.GetMousePosition` (`GameplayStatics.GetPlayerController` 0)))
  (if (`self.IsActorInspect`)
    (bind _output_get (set `self.RotHelper` (`KismetMathLibrary.RInterpTo` (`self.RotHelper`) (`KismetMathLibrary.MakeRotator` (* (- (/ _locationx _returnvalue_x) 0.5) 120.0) (* (- (/ _locationy _returnvalue_y) 0.5) -120.0)) DeltaTime 2.0)))
    (bind _output_get_2 (set `self.TargetRot` (`KismetMathLibrary.ComposeRotators` _output_get (`self.TargetBaseRot`))))
    (`self.K2_SetActorRotation` _output_get_2)))

(fn `IsInspectable`
  (returns (Yes :type Boolean))
  (return true))

(fn `SetBeeKiss`
  (params (IsKiss :type Boolean))
  (bind _asabp_bee (cast `/Game/BeeKeeper/Meshes/Bee/ABP_Bee` (`SkeletalMeshComponent.GetAnimInstance` (`self.BeeSKM`))))
  (set `/Game/BeeKeeper/Meshes/Bee/ABP_Bee.IsKiss` IsKiss _asabp_bee))

(fn `SetBeeTaken`
  (params (IsTaken :type Boolean))
  (bind _asabp_bee (cast `/Game/BeeKeeper/Meshes/Bee/ABP_Bee` (`SkeletalMeshComponent.GetAnimInstance` (`self.BeeSKM`))))
  (set `/Game/BeeKeeper/Meshes/Bee/ABP_Bee.IsTaken` IsTaken _asabp_bee))

(fn `ShowCrown`
  (`SceneComponent.SetVisibility` (`self.Crown`) true false))

(fn `SimAct`
  (params (Dt :type "Float (double-precision)"))
  (locals (EnableDebug :type Boolean))
  (bind _arrow (`self.Arrow`))
  (bind _simradius (`self.SimRadius`))
  (bind _velcoity (`self.Velcoity`))
  (bind _simheight (`self.SimHeight`))
  (bind _returnvalue (`KismetMathLibrary.Normal` (`self.Velcoity`)))
  (bind _x (.x (`self.BasePoint`)))
  (bind _y (.y (`self.BasePoint`)))
  (bind _z (.z (`self.BasePoint`)))
  (bind _returnvalue_2 (- (`self.NextPosPoint`) (`self.K2_GetActorLocation`)))
  (bind _returnvalue_3 (`KismetMathLibrary.Normal` (- (`self.NextPosPoint`) (`self.K2_GetActorLocation`))))
  (bind (_returnvalue_roll _returnvalue_pitch _returnvalue_yaw) (`KismetMathLibrary.BreakRotator` (`KismetMathLibrary.Conv_VectorToRotator` (`KismetMathLibrary.Normal` (`self.Velcoity`)))))
  (bind _returnvalue_4 (`KismetMathLibrary.VSize` _returnvalue_2))
  (bind (_returnvalue_x _returnvalue_y _returnvalue_z) (`KismetMathLibrary.BreakVector` (`KismetMathLibrary.Cross_VectorVector` _returnvalue_3 _returnvalue)))
  (bind _returnvalue_5 (`KismetMathLibrary.Dot_VectorVector` _returnvalue_3 _returnvalue))
  (bind _returnvalue_6 (* (`KismetMathLibrary.SignOfFloat` _returnvalue_z) -1.0))
  (if (`self.IsSimulationActive`)
    (`|ExecutionSequence`
      (:`then_0`
        (set `self.InterpVelSpeed` (`KismetMathLibrary.FInterpTo` (`self.InterpVelSpeed`) (`KismetMathLibrary.FClamp` (/ _returnvalue_4 (`self.ToPointLenght`) 0.3) 0.8 1.1) (`local.Dt`) 1.0))
        (set `self.Velcoity` (`KismetMathLibrary.ClampVectorSize` (+ (`KismetMathLibrary.VInterpTo` (`self.Velcoity`) (* (`KismetMathLibrary.Normal` _returnvalue_2) (`KismetMathLibrary.FClamp` (* _returnvalue_4 0.8) 0.0 100.0) 1.0) (`local.Dt`) (`self.InterpVelSpeed`)) (`KismetMathLibrary.VLerp` (0.0 0.0 0.0) (* (`self.GetActorRightVector`) _returnvalue_6 (`local.Dt`) 200.0) (`KismetMathLibrary.FClamp` (/ (+ _returnvalue_5 -0.5) -1.5)))) 0.0 100.0))
        (`self.K2_AddActorWorldOffset` (* (`self.Velcoity`) (`local.Dt`)))
        (`self.K2_SetActorRotation` (`KismetMathLibrary.RInterpTo` (`self.K2_GetActorRotation`) (`KismetMathLibrary.MakeRotator` _returnvalue_roll (+ _returnvalue_pitch (`KismetMathLibrary.Lerp` 0.0 -15.0 (/ (`KismetMathLibrary.VSize` (`self.Velcoity`)) 100.0))) _returnvalue_yaw) (`local.Dt`) 3.0)))
      (:`then_1`
        (if (`local.EnableDebug`)
          (`SceneComponent.SetHiddenInGame` _arrow false false)
          (`SceneComponent.K2_SetWorldRotation` _arrow (`KismetMathLibrary.Conv_VectorToRotator` (`KismetMathLibrary.Normal` _velcoity)) false false)
          (set `ArrowComponent.ArrowLength` (`KismetMathLibrary.VSize` _velcoity) _arrow)
          (`KismetSystemLibrary.DrawDebugSphere` (`self.NextPosPoint`) 5.0 12 (struct :`R` 1.0 :`A` 1.0))
          (`KismetSystemLibrary.PrintString` (`KismetStringLibrary.Conv_VectorToString` (0.0 0.0 0.0)) true true (struct :`G` 0.66 :`B` 1.0 :`A` 1.0) 0.0)))
      (:`then_2`
        (if (< (`KismetMathLibrary.VSize` (- (`self.NextPosPoint`) (`self.K2_GetActorLocation`))) 10.0)
          (set `self.NextPosPoint` (`KismetMathLibrary.MakeVector` (`KismetMathLibrary.RandomFloatInRange` (- _x _simradius) (+ _x _simradius)) (`KismetMathLibrary.RandomFloatInRange` (- _y _simradius) (+ _y _simradius)) (`KismetMathLibrary.RandomFloatInRange` (- _z _simheight) (+ _z _simheight))))
          (set `self.ToPointLenght` (`KismetMathLibrary.VSize` (- (`self.NextPosPoint`) (`self.K2_GetActorLocation`))))))
      (:`then_3`
        (set `self.VelRig` (`KismetMathLibrary.MakeVector` (/ (`KismetMathLibrary.VSize` (`self.Velcoity`)) -100.0) (* _returnvalue_6 (- (`KismetMathLibrary.Abs` _returnvalue_5) 1.0))))))))

(fn `Update Mesh Species`
  (params (species :type "Species Enum" :default "Meadow"))
  (bind _returnvalue (`|GetDataTableRow` "/Game/BeeKeeper/BeeModel/DT_Icons.DT_Icons" (`|GetEnumeratorName` species))
    (:`then`
      (`self.UpdateMaterials` (`KismetMathLibrary.Conv_ColorToLinearColor` (`.Main` (break `Icon` _returnvalue))) (`KismetMathLibrary.Conv_ColorToLinearColor` (`.MainDark` (break `Icon` _returnvalue))) (`KismetMathLibrary.Conv_ColorToLinearColor` (`.Sec` (break `Icon` _returnvalue)))))
    (:`RowNotFound`
      (bind _returnvalue_2 (`|GetDataTableRow` "/Game/BeeKeeper/BeeModel/DT_Icons.DT_Icons" "Meadow")
        (:`then`
          (`self.UpdateMaterials` (`KismetMathLibrary.Conv_ColorToLinearColor` (`.Main` (break `Icon` _returnvalue_2))) (`KismetMathLibrary.Conv_ColorToLinearColor` (`.MainDark` (break `Icon` _returnvalue_2))) (`KismetMathLibrary.Conv_ColorToLinearColor` (`.Sec` (break `Icon` _returnvalue_2)))))))))

(fn `UpdateBeeProps`
  (params (Bee :type "BeeGenetic Object Reference") (AddTagName :type Name :default "BeeProp"))
  (bind _returnvalue (`InheritMutationLibrary.CopyBeeProps` Bee))
  (bind _output_get (set `self.BeeGenetic` _returnvalue))
  (`self.UpdateBeeInfo`)
  (`self.Update Mesh Species` (`BeeGenetic.Main` _output_get))
  (`KismetArrayLibrary.Array_AddUnique` (`self.Tags`) AddTagName)
  (if (`self.IsActorSpawn`)
    (`self.SetActorEnableCollision` true)))

(fn `UpdateMaterials`
  (params (Main :type "LinearColor Structure" :default (struct :`R` 0.803922 :`G` 0.231373)) (MainDark :type "LinearColor Structure" :default (struct :`R` 0.27451 :`G` 0.094118)) (Sec :type "LinearColor Structure" :default (struct :`R` 0.031373 :`G` 0.031373 :`B` 0.031373)))
  (`MaterialInstanceDynamic.SetVectorParameterValue` (`self.MainMat`) "MainColor" (`local.Main`))
  (`MaterialInstanceDynamic.SetVectorParameterValue` (`self.MainMat`) "SecColor" (`local.Sec`)))

(fn `UserConstructionScript`
  (bind (_returnvalue_year _returnvalue_month _returnvalue_day) (`KismetMathLibrary.BreakDateTime` (`KismetMathLibrary.Now`)))
  (bind _returnvalue (`PrimitiveComponent.CreateDynamicMaterialInstance` (`self.BeeSKM`) 0 null "None"))
  (set `self.MainMat` _returnvalue)
  (`SceneComponent.SetVisibility` (`self.Hat`) (or (and (== _returnvalue_month 12) (> _returnvalue_day 14)) (and (== _returnvalue_month 1) (<= _returnvalue_day 31))) false))